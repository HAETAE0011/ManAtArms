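; Simplex_BP is an actor that represents a four-point simplex as a moving, spinning mesh.
; Each tick it moves along its forward arrow without sweep and manually integrates angular velocity into a normalized quaternion, applied to the static mesh with the starting rotation as offset.
; Helper functions capture the four point components' world locations as vertices, replace one by index, and return their centroid.
; The Support function is an empty stub.
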(event EventBeginPlay
  ;[1 1 1] Initializing offset
  (Variables|Default|SetInitialRotation (Transformation|GetActorRotation)))

(event EventTick
  (params (DeltaSeconds :type Float%20%28single-precision%29))
  (bind _returnvalue (Math|Trig|GetPI))
  (bind _returnvalue_2 (/ DeltaSeconds 2.0))
  (bind _angularvel (Variables|Default|GetangularVel))
  (bind _returnvalue_3 (* _angularvel _returnvalue))
  (bind _returnvalue_4 (/ _returnvalue_3 1.8e+02))
  ;[1 1 1] Base Movement
  ;;[0 1 0.4588] move forward function
  (Transformation|SetActorLocation (+ (Transformation|GetActorLocation) (* (Math|Vector|GetForwardVector (Variables|Default|GetForwardArrow)) (* DeltaSeconds (Variables|Default|GetVelocityMultiplier)))) false false)
  ;;[1 0.4556 0.3051] Angular Velocity set
  (Variables|Default|SetAngularVelocity (Utilities|Struct|MakeQuat 0.0 (.x _returnvalue_4) (.y _returnvalue_4) (.z _returnvalue_4)))
  ;;[0.05071 0.1095 0.1562] Normalize
  (bind _output_get (Variables|Default|SetOrientation (Class|KismetMathLibrary|QuatNormalized (+ (Variables|Default|GetOrientation) (Utilities|Struct|MakeQuat (* (.X (Utilities|Struct|BreakQuat (* (Variables|Default|GetOrientation) (Variables|Default|GetAngularVelocity)))) _returnvalue_2) (* (.Y (Utilities|Struct|BreakQuat (* (Variables|Default|GetOrientation) (Variables|Default|GetAngularVelocity)))) _returnvalue_2) (* (.Z (Utilities|Struct|BreakQuat (* (Variables|Default|GetOrientation) (Variables|Default|GetAngularVelocity)))) _returnvalue_2) (* (.W (Utilities|Struct|BreakQuat (* (Variables|Default|GetOrientation) (Variables|Default|GetAngularVelocity)))) _returnvalue_2))) 1e-06)))
  (Transformation|SetRelativeRotation (Variables|Default|GetStaticMesh) (Math|Rotator|CombineRotators (Variables|Default|GetInitialRotation) (Class|KismetMathLibrary|QuatRotator _output_get)) false false))

(fn ConstructionScript)

(fn Support)

(fn GetCentre
  (return (/ (+ (Variables|Default|GetVertexPoint1) (Variables|Default|GetVertexPoint2) (Variables|Default|GetVertexPoint3) (Variables|Default|GetVertexPoint4)) 4.0)))

(fn ModifyPoint
  (params (pointToChange :type Integer) (newVector :type Vector))
  (switch int pointToChange
    (:1
      (Variables|Default|SetVertexPoint1 newVector))
    (:2
      (Variables|Default|SetVertexPoint2 newVector))
    (:3
      (Variables|Default|SetVertexPoint3 newVector))
    (:4
      (Variables|Default|SetVertexPoint4 newVector))))

(fn Initialize
  (Variables|Default|SetVertexPoint1 (Transformation|GetWorldLocation (Variables|Default|Getpoint1)))
  (Variables|Default|SetVertexPoint2 (Transformation|GetWorldLocation (Variables|Default|Getpoint2)))
  (Variables|Default|SetVertexPoint3 (Transformation|GetWorldLocation (Variables|Default|Getpoint3)))
  (Variables|Default|SetVertexPoint4 (Transformation|GetWorldLocation (Variables|Default|Getpoint4))))