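; GJK collision test between two four-point Simplex objects, run from the construction script after overwriting their vertices with hard-coded points.
; Support points along successive directions form a Minkowski-difference tetrahedron A-B-C-D.
; Determinant sign comparisons check whether it contains the origin, setting GotCollision and printing debug output.
; Instead of looping, a failed check gets one retry, replacing B using the ACD face normal.
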(event EventBeginPlay)

(event Collision|EventActorBeginOverlap
  (params (OtherActor :type Actor%20Object%20Reference)))

(event EventTick
  (params (DeltaSeconds :type Float%20%28single-precision%29)))

(fn ConstructionScript
  (if (Variables|Default|Getrefresh)
    (Variables|Default|Setrefresh false))
  (CallFunction|IsColliding?))

(fn IsColliding?
  (bind _returnvalue (|Do_2))
  (bind _returnvalue_2 (|D3_2))
  (bind _returnvalue_3 (|Do))
  (bind _simplex1 (Variables|Default|GetSimplex1))
  (bind _simplex2 (Variables|Default|GetSimplex2))
  (bind _simplex1_2 (Variables|Default|GetSimplex1))
  (bind _simplex2_2 (Variables|Default|GetSimplex2))
  (bind _simplex1_3 (Variables|Default|GetSimplex1))
  (bind _simplex1_4 (Variables|Default|GetSimplex1))
  (bind _simplex2_3 (Variables|Default|GetSimplex2))
  (bind _simplex2_4 (Variables|Default|GetSimplex2))
  (bind _simplex1_5 (Variables|Default|GetSimplex1))
  (bind _simplex2_5 (Variables|Default|GetSimplex2))
  (bind _simplex1_6 (Variables|Default|GetSimplex1))
  (bind _simplex2_6 (Variables|Default|GetSimplex2))
  (bind _returnvalue_4 (* _returnvalue _returnvalue_2))
  (bind _vertexpoint2 (Variables|/Game/MyContent/Assginment/Simplex_BP.Simplex_BP_C|GetVertexPoint2 _simplex2_4))
  (bind _vertexpoint3 (Variables|/Game/MyContent/Assginment/Simplex_BP.Simplex_BP_C|GetVertexPoint3 _simplex2_4))
  (bind _vertexpoint4 (Variables|/Game/MyContent/Assginment/Simplex_BP.Simplex_BP_C|GetVertexPoint4 _simplex2_4))
  (bind _vertexpoint1 (Variables|/Game/MyContent/Assginment/Simplex_BP.Simplex_BP_C|GetVertexPoint1 _simplex1_2))
  (bind _vertexpoint2_2 (Variables|/Game/MyContent/Assginment/Simplex_BP.Simplex_BP_C|GetVertexPoint2 _simplex1_2))
  (bind _vertexpoint3_2 (Variables|/Game/MyContent/Assginment/Simplex_BP.Simplex_BP_C|GetVertexPoint3 _simplex1_2))
  (bind _vertexpoint4_2 (Variables|/Game/MyContent/Assginment/Simplex_BP.Simplex_BP_C|GetVertexPoint4 _simplex1_2))
  (bind _vertexpoint1_2 (Variables|/Game/MyContent/Assginment/Simplex_BP.Simplex_BP_C|GetVertexPoint1 _simplex2_2))
  (bind _vertexpoint2_3 (Variables|/Game/MyContent/Assginment/Simplex_BP.Simplex_BP_C|GetVertexPoint2 _simplex2_2))
  (bind _vertexpoint3_3 (Variables|/Game/MyContent/Assginment/Simplex_BP.Simplex_BP_C|GetVertexPoint3 _simplex2_2))
  (bind _vertexpoint4_3 (Variables|/Game/MyContent/Assginment/Simplex_BP.Simplex_BP_C|GetVertexPoint4 _simplex2_2))
  (bind _vertexpoint1_3 (Variables|/Game/MyContent/Assginment/Simplex_BP.Simplex_BP_C|GetVertexPoint1 _simplex1_3))
  (bind _vertexpoint1_4 (Variables|/Game/MyContent/Assginment/Simplex_BP.Simplex_BP_C|GetVertexPoint1 _simplex1_4))
  (bind _vertexpoint2_4 (Variables|/Game/MyContent/Assginment/Simplex_BP.Simplex_BP_C|GetVertexPoint2 _simplex1_4))
  (bind _vertexpoint3_4 (Variables|/Game/MyContent/Assginment/Simplex_BP.Simplex_BP_C|GetVertexPoint3 _simplex1_4))
  (bind _vertexpoint4_4 (Variables|/Game/MyContent/Assginment/Simplex_BP.Simplex_BP_C|GetVertexPoint4 _simplex1_4))
  (bind _vertexpoint1_5 (Variables|/Game/MyContent/Assginment/Simplex_BP.Simplex_BP_C|GetVertexPoint1 _simplex2_3))
  (bind _vertexpoint2_5 (Variables|/Game/MyContent/Assginment/Simplex_BP.Simplex_BP_C|GetVertexPoint2 _simplex1_3))
  (bind _vertexpoint2_6 (Variables|/Game/MyContent/Assginment/Simplex_BP.Simplex_BP_C|GetVertexPoint2 _simplex2_3))
  (bind _vertexpoint3_5 (Variables|/Game/MyContent/Assginment/Simplex_BP.Simplex_BP_C|GetVertexPoint3 _simplex2_3))
  (bind _vertexpoint4_5 (Variables|/Game/MyContent/Assginment/Simplex_BP.Simplex_BP_C|GetVertexPoint4 _simplex2_3))
  (bind _vertexpoint3_6 (Variables|/Game/MyContent/Assginment/Simplex_BP.Simplex_BP_C|GetVertexPoint3 _simplex1_3))
  (bind _vertexpoint4_6 (Variables|/Game/MyContent/Assginment/Simplex_BP.Simplex_BP_C|GetVertexPoint4 _simplex1_3))
  (bind _vertexpoint1_6 (Variables|/Game/MyContent/Assginment/Simplex_BP.Simplex_BP_C|GetVertexPoint1 _simplex1_5))
  (bind _vertexpoint2_7 (Variables|/Game/MyContent/Assginment/Simplex_BP.Simplex_BP_C|GetVertexPoint2 _simplex1_5))
  (bind _vertexpoint3_7 (Variables|/Game/MyContent/Assginment/Simplex_BP.Simplex_BP_C|GetVertexPoint3 _simplex1_5))
  (bind _vertexpoint4_7 (Variables|/Game/MyContent/Assginment/Simplex_BP.Simplex_BP_C|GetVertexPoint4 _simplex1_5))
  (bind _vertexpoint1_7 (Variables|/Game/MyContent/Assginment/Simplex_BP.Simplex_BP_C|GetVertexPoint1 _simplex2_5))
  (bind _vertexpoint2_8 (Variables|/Game/MyContent/Assginment/Simplex_BP.Simplex_BP_C|GetVertexPoint2 _simplex2_5))
  (bind _vertexpoint3_8 (Variables|/Game/MyContent/Assginment/Simplex_BP.Simplex_BP_C|GetVertexPoint3 _simplex2_5))
  (bind _vertexpoint4_8 (Variables|/Game/MyContent/Assginment/Simplex_BP.Simplex_BP_C|GetVertexPoint4 _simplex2_5))
  (bind _vertexpoint1_8 (Variables|/Game/MyContent/Assginment/Simplex_BP.Simplex_BP_C|GetVertexPoint1 _simplex1_6))
  (bind _vertexpoint2_9 (Variables|/Game/MyContent/Assginment/Simplex_BP.Simplex_BP_C|GetVertexPoint2 _simplex1_6))
  (bind _vertexpoint3_9 (Variables|/Game/MyContent/Assginment/Simplex_BP.Simplex_BP_C|GetVertexPoint3 _simplex1_6))
  (bind _vertexpoint4_9 (Variables|/Game/MyContent/Assginment/Simplex_BP.Simplex_BP_C|GetVertexPoint4 _simplex1_6))
  (bind _vertexpoint1_9 (Variables|/Game/MyContent/Assginment/Simplex_BP.Simplex_BP_C|GetVertexPoint1 _simplex2_6))
  (bind _vertexpoint2_10 (Variables|/Game/MyContent/Assginment/Simplex_BP.Simplex_BP_C|GetVertexPoint2 _simplex2_6))
  (bind _vertexpoint3_10 (Variables|/Game/MyContent/Assginment/Simplex_BP.Simplex_BP_C|GetVertexPoint3 _simplex2_6))
  (bind _vertexpoint4_10 (Variables|/Game/MyContent/Assginment/Simplex_BP.Simplex_BP_C|GetVertexPoint4 _simplex2_6))
  (bind _vertexpoint1_10 (Variables|/Game/MyContent/Assginment/Simplex_BP.Simplex_BP_C|GetVertexPoint1 _simplex2_4))
  (Utilities|IsValid _simplex1
    (:Is%20Valid
      (Utilities|IsValid _simplex2
        (:Is%20Valid
          (Default|Initialize _simplex1)
          (Default|Initialize _simplex2)
          (CallFunction|ChangePointValues "0.500000,0.800000,0.300000" "0.000000,0.000000,0.000000" "0.500000,0.000000,0.900000" "1.000000,0.000000,0.000000" "0.500000,0.100000,0.300000" "0.000000,-0.700000,0.000000" "0.500000,-0.700000,0.900000" "1.000000,-0.700000,0.000000")
          ;[1 1 1] Get Centre
          (bind _centre (Default|GetCentre _simplex1))
          (Variables|Default|Setcentre1 _centre)
          (bind _centre_2 (Default|GetCentre _simplex2))
          (Variables|Default|Setcentre2 _centre_2)
          ;[1 1 1] direction D
          (Variables|Default|SetDirection (Math|Vector|Normalize (- (Variables|Default|Getcentre2) (Variables|Default|Getcentre1))))
          ;[1 1 1] Project each shape Si along d
          (Variables|Default|SetP1 (Utilities|Array|Get(acopy) (Utilities|Array|MakeArray _vertexpoint1_6 _vertexpoint2_7 _vertexpoint3_7 _vertexpoint4_7) (.IndexOfMaxValue (Math|Float|MaxOfFloatArray (Utilities|Array|MakeArray (Math|Vector|DotProduct _vertexpoint1_6 (Variables|Default|GetDirection)) (Math|Vector|DotProduct _vertexpoint2_7 (Variables|Default|GetDirection)) (Math|Vector|DotProduct _vertexpoint3_7 (Variables|Default|GetDirection)) (Math|Vector|DotProduct _vertexpoint4_7 (Variables|Default|GetDirection)))))))
          (Variables|Default|SetP2 (Utilities|Array|Get(acopy) (Utilities|Array|MakeArray _vertexpoint1_7 _vertexpoint2_8 _vertexpoint3_8 _vertexpoint4_8) (.IndexOfMinValue (Math|Float|MinOfFloatArray (Utilities|Array|MakeArray (Math|Vector|DotProduct _vertexpoint1_7 (Variables|Default|GetDirection)) (Math|Vector|DotProduct _vertexpoint2_8 (Variables|Default|GetDirection)) (Math|Vector|DotProduct _vertexpoint3_8 (Variables|Default|GetDirection)) (Math|Vector|DotProduct _vertexpoint4_8 (Variables|Default|GetDirection)))))))
          ;[1 1 1] Minkowski difference: This is the first point of the simplex
          (bind _output_get (Variables|Default|Seta (- (Variables|Default|GetP1) (Variables|Default|GetP2))))
          ;[1 1 1] direction D in opposite direction
          (Variables|Default|SetDirection (Math|Vector|Normalize (- (Variables|Default|Getcentre1) (Variables|Default|Getcentre2))))
          ;[1 1 1] Project each shape Si along new d
          (Variables|Default|SetP1 (Utilities|Array|Get(acopy) (Utilities|Array|MakeArray _vertexpoint1_3 _vertexpoint2_5 _vertexpoint3_6 _vertexpoint4_6) (.IndexOfMaxValue (Math|Float|MaxOfFloatArray (Utilities|Array|MakeArray (Math|Vector|DotProduct _vertexpoint1_3 (Variables|Default|GetDirection)) (Math|Vector|DotProduct _vertexpoint2_5 (Variables|Default|GetDirection)) (Math|Vector|DotProduct _vertexpoint3_6 (Variables|Default|GetDirection)) (Math|Vector|DotProduct _vertexpoint4_6 (Variables|Default|GetDirection)))))))
          (Variables|Default|SetP2 (Utilities|Array|Get(acopy) (Utilities|Array|MakeArray _vertexpoint1_10 _vertexpoint2 _vertexpoint3 _vertexpoint4) (.IndexOfMinValue (Math|Float|MinOfFloatArray (Utilities|Array|MakeArray (Math|Vector|DotProduct _vertexpoint1_10 (Variables|Default|GetDirection)) (Math|Vector|DotProduct _vertexpoint2 (Variables|Default|GetDirection)) (Math|Vector|DotProduct _vertexpoint3 (Variables|Default|GetDirection)) (Math|Vector|DotProduct _vertexpoint4 (Variables|Default|GetDirection)))))))
          ;[1 1 1] Minkowski difference: This is the second point of the simplex
          (bind _output_get_2 (Variables|Default|Setb (- (Variables|Default|GetP1) (Variables|Default|GetP2))))
          ;[1 1 1] New direction which is perpendicular to the line segment ab towards the origin
          (Variables|Default|SetDirection (Math|Vector|CrossProduct (Math|Vector|CrossProduct (- (Variables|Default|Getb) (Variables|Default|Geta)) (- "0, 0, 0" (Variables|Default|Geta))) (- (Variables|Default|Getb) (Variables|Default|Geta))))
          ;[1 1 1] Project each shape Si along d
          (Variables|Default|SetP1 (Utilities|Array|Get(acopy) (Utilities|Array|MakeArray _vertexpoint1 _vertexpoint2_2 _vertexpoint3_2 _vertexpoint4_2) (.IndexOfMaxValue (Math|Float|MaxOfFloatArray (Utilities|Array|MakeArray (Math|Vector|DotProduct _vertexpoint1 (Variables|Default|GetDirection)) (Math|Vector|DotProduct _vertexpoint2_2 (Variables|Default|GetDirection)) (Math|Vector|DotProduct _vertexpoint3_2 (Variables|Default|GetDirection)) (Math|Vector|DotProduct _vertexpoint4_2 (Variables|Default|GetDirection)))))))
          (Variables|Default|SetP2 (Utilities|Array|Get(acopy) (Utilities|Array|MakeArray _vertexpoint1_2 _vertexpoint2_3 _vertexpoint3_3 _vertexpoint4_3) (.IndexOfMinValue (Math|Float|MinOfFloatArray (Utilities|Array|MakeArray (Math|Vector|DotProduct _vertexpoint1_2 (Variables|Default|GetDirection)) (Math|Vector|DotProduct _vertexpoint2_3 (Variables|Default|GetDirection)) (Math|Vector|DotProduct _vertexpoint3_3 (Variables|Default|GetDirection)) (Math|Vector|DotProduct _vertexpoint4_3 (Variables|Default|GetDirection)))))))
          ;[1 1 1] Minkowski difference: This is the third point of the simplex
          (Variables|Default|Setc (- (Variables|Default|GetP1) (Variables|Default|GetP2)))
          ;[1 1 1] N
          (Variables|Default|SetN1 (Math|Vector|CrossProduct (- (Variables|Default|Getb) (Variables|Default|Geta)) (- (Variables|Default|Getc) (Variables|Default|Geta))))
          (Variables|Default|SetN2 (* (Math|Vector|CrossProduct (- (Variables|Default|Getb) (Variables|Default|Geta)) (- (Variables|Default|Getc) (Variables|Default|Geta))) -1.0))
          (if (> (Math|Vector|DotProduct (Variables|Default|GetN1) (- "0, 0, 0" (/ (+ (Variables|Default|Geta) (Variables|Default|Getb) (Variables|Default|Getc)) 3.0))) 0.0)
            (Variables|Default|SetN (Variables|Default|GetN1))
            (else
              (Variables|Default|SetN (Variables|Default|GetN2))))
          ;[1 1 1] Project each shape Si along d
          (Variables|Default|SetP1 (Utilities|Array|Get(acopy) (Utilities|Array|MakeArray _vertexpoint1_4 _vertexpoint2_4 _vertexpoint3_4 _vertexpoint4_4) (.IndexOfMaxValue (Math|Float|MaxOfFloatArray (Utilities|Array|MakeArray (Math|Vector|DotProduct _vertexpoint1_4 (Variables|Default|GetN)) (Math|Vector|DotProduct _vertexpoint2_4 (Variables|Default|GetN)) (Math|Vector|DotProduct _vertexpoint3_4 (Variables|Default|GetN)) (Math|Vector|DotProduct _vertexpoint4_4 (Variables|Default|GetN)))))))
          (Variables|Default|SetP2 (Utilities|Array|Get(acopy) (Utilities|Array|MakeArray _vertexpoint1_5 _vertexpoint2_6 _vertexpoint3_5 _vertexpoint4_5) (.IndexOfMinValue (Math|Float|MinOfFloatArray (Utilities|Array|MakeArray (Math|Vector|DotProduct _vertexpoint1_5 (Variables|Default|GetN)) (Math|Vector|DotProduct _vertexpoint2_6 (Variables|Default|GetN)) (Math|Vector|DotProduct _vertexpoint3_5 (Variables|Default|GetN)) (Math|Vector|DotProduct _vertexpoint4_5 (Variables|Default|GetN)))))))
          ;[1 1 1] Minkowski difference: This is the forth point of the simplex
          (Variables|Default|Setd (- (Variables|Default|GetP1) (Variables|Default|GetP2)))
          (if (Math|Boolean|ANDBoolean (>= (* _returnvalue_3 (|D1)) 0.0) (>= (* _returnvalue_3 (|D2)) 0.0) (>= (* _returnvalue_3 (|D3)) 0.0) (>= (* _returnvalue_3 (|D4)) 0.0))
            (Variables|Default|SetGotCollision! true)
            (Development|PrintString "col")
            (else
              (Variables|Default|SetGotCollision! false)
              ;[1 1 1] N
              (Variables|Default|SetN1 (Math|Vector|CrossProduct (- (Variables|Default|Getc) (Variables|Default|Geta)) (- (Variables|Default|Getd) (Variables|Default|Geta))))
              (Variables|Default|SetN2 (* (Math|Vector|CrossProduct (- (Variables|Default|Getc) (Variables|Default|Geta)) (- (Variables|Default|Getd) (Variables|Default|Geta))) -1.0))
              (if (> (Math|Vector|DotProduct (Variables|Default|GetN1) (- "0, 0, 0" (/ (+ (Variables|Default|Geta) (Variables|Default|Getb) (Variables|Default|Getd)) 3.0))) 0.0)
                (Variables|Default|SetN (Variables|Default|GetN1))
                (else
                  (Variables|Default|SetN (Variables|Default|GetN2))))
              ;[1 1 1] Project each shape Si along d
              (Variables|Default|SetP1 (Utilities|Array|Get(acopy) (Utilities|Array|MakeArray _vertexpoint1_8 _vertexpoint2_9 _vertexpoint3_9 _vertexpoint4_9) (.IndexOfMaxValue (Math|Float|MaxOfFloatArray (Utilities|Array|MakeArray (Math|Vector|DotProduct _vertexpoint1_8 (Variables|Default|GetN)) (Math|Vector|DotProduct _vertexpoint2_9 (Variables|Default|GetN)) (Math|Vector|DotProduct _vertexpoint3_9 (Variables|Default|GetN)) (Math|Vector|DotProduct _vertexpoint4_9 (Variables|Default|GetN)))))))
              (Variables|Default|SetP2 (Utilities|Array|Get(acopy) (Utilities|Array|MakeArray _vertexpoint1_9 _vertexpoint2_10 _vertexpoint3_10 _vertexpoint4_10) (.IndexOfMinValue (Math|Float|MinOfFloatArray (Utilities|Array|MakeArray (Math|Vector|DotProduct _vertexpoint1_9 (Variables|Default|GetN)) (Math|Vector|DotProduct _vertexpoint2_10 (Variables|Default|GetN)) (Math|Vector|DotProduct _vertexpoint3_10 (Variables|Default|GetN)) (Math|Vector|DotProduct _vertexpoint4_10 (Variables|Default|GetN)))))))
              ;[1 1 1] Minkowski difference: This is the forth point of the simplex
              (Variables|Default|Setb (- (Variables|Default|GetP1) (Variables|Default|GetP2)))
              (if (Math|Boolean|ANDBoolean (>= (* _returnvalue (|D1_2)) 0.0) (>= (* _returnvalue (|D2_2)) 0.0) (>= _returnvalue_4 0.0) (>= (* _returnvalue (|D4_2)) 0.0))
                (Variables|Default|SetGotCollision! true)
                (Development|PrintString "col")
                (else
                  (Variables|Default|SetGotCollision! false)
                  (Development|PrintString (Utilities|String|ToString(Float) _returnvalue_4)))))))))))

(fn ChangePointValues
  (params (point1 :type Vector) (point2 :type Vector) (point3 :type Vector) (point4 :type Vector) (point5 :type Vector) (point6 :type Vector) (point7 :type Vector) (point8 :type Vector))
  (bind _simplex2 (Variables|Default|GetSimplex2))
  (bind _simplex1 (Variables|Default|GetSimplex1))
  (Default|ModifyPoint _simplex1 1 point1)
  (Default|ModifyPoint _simplex1 2 point2)
  (Default|ModifyPoint _simplex1 3 point3)
  (Default|ModifyPoint _simplex1 4 point4)
  (Default|ModifyPoint _simplex2 1 point5)
  (Default|ModifyPoint _simplex2 2 point6)
  (Default|ModifyPoint _simplex2 3 point7)
  (Default|ModifyPoint _simplex2 4 point8))