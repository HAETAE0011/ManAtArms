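; Actor that builds a grid of pathfinding nodes over a box area and runs A* across it every three seconds.
; Construction sphere-traces and debug-draws each cell's availability; BeginPlay spawns a BP_Node per cell.
; FindPath searches eight-way neighbours using straight-line G/H costs, linking parents for ReTracePath's indicator spawning.
; Location-to-node lookup is unfinished, and ReTracePath only enters its trace when start equals end, so paths are never rebuilt.
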(event EventBeginPlay
  (bind _nodes_loc (Variables|grid|GetNodes_Loc))
  (for _index (range 0 (- (Utilities|Array|Length _nodes_loc) 1))
    (bind _returnvalue (Game|SpawnActorfromClass "/Game/MyContent/BP/AI/BP_Node.BP_Node_C" (Math|Transform|MakeTransform (Utilities|Array|Get(acopy) _nodes_loc _index) (Transformation|GetActorRotation) "1,1,1") "AlwaysSpawn" 0 0))
    (Variables|/Game/MyContent/BP/AI/BP_Node.BP_Node_C|Setnum _returnvalue _index)
    (Utilities|Array|Add (Variables|grid|GetNodes) _returnvalue)))

(event EventTick
  (params (DeltaSeconds :type Float%20%28single-precision%29))
  (bind _output_get (Variables|Default|Setcounter (- (Variables|Default|Getcounter) DeltaSeconds)))
  (if (<= _output_get 0.0)
    (CallFunction|FindPath)
    (Variables|Default|Setcounter 3.0)))

(fn ConstructionScript
  (bind _returnvalue (Transformation|GetActorRotation))
  (bind _returnvalue_2 (Transformation|GetActorLocation))
  (bind _numofnodes_x (Variables|grid|GetNumOfNodes_X))
  ;[1 1 1] Refresh
  (if (Variables|grid|GetRefresh)
    (Variables|grid|SetRefresh false))
  ;[1 1 1] Set width&length
  (Components|Box|SetBoxExtent (Variables|Default|GetArea) (Math|Vector|MakeVector (Variables|grid|GetWidth) (Variables|grid|GetLength) 1e+01) true)
  (Variables|grid|SetNodeSize_w (/ (Variables|grid|GetWidth) (Math|Conversions|ToFloat(Integer) (Variables|grid|GetNumOfNodes_X))))
  (Variables|grid|SetNodeSize_l (/ (Variables|grid|GetLength) (Math|Conversions|ToFloat(Integer) (Variables|grid|GetNumOfNodes_Y))))
  ;[1 1 1] Nodes
  (Utilities|Array|Clear (Variables|grid|GetNodes_Loc))
  (Utilities|Array|Clear (Variables|grid|GetNodes_availability))
  (Variables|grid|SetStartPoint (Math|Vector|MakeVector (+ (- (.x _returnvalue_2) (Variables|grid|GetWidth)) (Variables|grid|GetNodeSize_w)) (+ (- (.y _returnvalue_2) (Variables|grid|GetLength)) (Variables|grid|GetNodeSize_l)) (.z _returnvalue_2)))
  (for _index (range 0 (- (Variables|grid|GetNumOfNodes_Y) 1))
    (for _index_2 (range 0 (- _numofnodes_x 1))
      (Utilities|Array|Add (Variables|grid|GetNodes_Loc) (+ (Variables|grid|GetStartPoint) (Math|Vector|MakeVector (* _index_2 (* (Variables|grid|GetNodeSize_w) 2.0)) (* _index (* (Variables|grid|GetNodeSize_l) 2.0)) 0.0)))
      (bind _returnvalue_3 (Collision|SphereTraceByChannel (Utilities|Array|Get(acopy) (Variables|grid|GetNodes_Loc) (+ (* _numofnodes_x _index) _index_2)) (Utilities|Array|Get(acopy) (Variables|grid|GetNodes_Loc) (+ (* _numofnodes_x _index) _index_2)) (* (Variables|grid|GetNodeSize_w) 0.95) "TraceTypeQuery1" false 0 "None"))
      (if _returnvalue_3
        (Rendering|Debug|DrawDebugBox (+ (Variables|grid|GetStartPoint) (Math|Vector|MakeVector (* _index_2 (* (Variables|grid|GetNodeSize_w) 2.0)) (* _index (* (Variables|grid|GetNodeSize_l) 2.0)) 0.0)) (Math|Vector|MakeVector (* (Variables|grid|GetNodeSize_w) 0.95) (* (Variables|grid|GetNodeSize_l) 0.95) 0.0) "(R=1.000000,G=0.000000,B=0.000000,A=1.000000)" _returnvalue 5e+01 0.0)
        (Utilities|Array|Add (Variables|grid|GetNodes_availability) false)
        (else
          (Rendering|Debug|DrawDebugBox (+ (Variables|grid|GetStartPoint) (Math|Vector|MakeVector (* _index_2 (* (Variables|grid|GetNodeSize_w) 2.0)) (* _index (* (Variables|grid|GetNodeSize_l) 2.0)) 0.0)) (Math|Vector|MakeVector (* (Variables|grid|GetNodeSize_w) 0.95) (* (Variables|grid|GetNodeSize_l) 0.95) 0.0) "(R=0.000000,G=0.147448,B=1.000000,A=1.000000)" _returnvalue 5e+01 0.0)
          (Utilities|Array|Add (Variables|grid|GetNodes_availability) true))))))

(fn NodefromLoc
  (params (Location :type Vector))
  (bind _returnvalue (Transformation|GetActorLocation))
  (bind _returnvalue_2 (- Location _returnvalue))
  (if (and (<= (Math|Float|Absolute(Float) (.x _returnvalue_2)) (Variables|grid|GetWidth)) (<= (Math|Float|Absolute(Float) (.y _returnvalue_2)) (Variables|grid|GetLength)))
    _))

(fn GetNeighbourNodes
  (params (Node :type BP%20Node%20Object%20Reference))
  (bind _nodes (Variables|grid|GetNodes))
  (bind _numofnodes_x (Variables|grid|GetNumOfNodes_X))
  (bind _returnvalue (Utilities|Array|FindItem _nodes Node))
  (bind _returnvalue_2 (Math|Integer|%(Integer) _returnvalue _numofnodes_x))
  (bind _returnvalue_3 (- _returnvalue _numofnodes_x))
  (bind _returnvalue_4 (== _returnvalue_3 0))
  (bind _returnvalue_5 (== _returnvalue_2 0))
  (Utilities|Array|Clear (Variables|grid|GetNeighbourArray))
  (if (Utilities|Array|IsValidIndex _nodes _returnvalue)
    (Utilities|FlowControl|Sequence
      (:then_0
        (if (not _returnvalue_4)
          (CallFunction|AddtoNeighbourArray (+ _returnvalue 1))))
      (:then_1
        (if (not _returnvalue_5)
          (CallFunction|AddtoNeighbourArray (- _returnvalue 1))))
      (:then_2
        (CallFunction|AddtoNeighbourArray (+ _returnvalue _numofnodes_x)))
      (:then_3
        (CallFunction|AddtoNeighbourArray (- _returnvalue _numofnodes_x)))
      (:then_4
        (if (not _returnvalue_4)
          (CallFunction|AddtoNeighbourArray (+ (+ _returnvalue _numofnodes_x) 1))))
      (:then_5
        (if (not _returnvalue_5)
          (CallFunction|AddtoNeighbourArray (- (+ _returnvalue _numofnodes_x) 1))))
      (:then_6
        (if (not _returnvalue_4)
          (CallFunction|AddtoNeighbourArray (+ (- _returnvalue _numofnodes_x) 1))))
      (:then_7
        (if (not _returnvalue_5)
          (CallFunction|AddtoNeighbourArray (- (- _returnvalue _numofnodes_x) 1))))
      (:then_8
        (return (Variables|grid|GetNeighbourArray))))))

(fn AddtoNeighbourArray
  (params (Index :type Integer))
  (bind _nodes (Variables|grid|GetNodes))
  (if (and (Utilities|Array|IsValidIndex _nodes Index) (Utilities|Array|Get(acopy) (Variables|grid|GetNodes_availability) Index))
    (Utilities|Array|Add (Variables|grid|GetNeighbourArray) (Utilities|Array|Get(acopy) _nodes Index))))

(fn LocfromNode
  (params (input%20Node :type BP%20Node%20Object%20Reference))
  (Utilities|IsValid input%20Node
    (:Is%20Valid
      (return (Variables|/Game/MyContent/BP/AI/BP_Node.BP_Node_C|GetLocation input%20Node)))))

(fn GetStartEndNodes
  (params (index1 :type Integer) (index2 :type Integer))
  (bind _nodes (Variables|grid|GetNodes))
  (return (Utilities|Array|Get(acopy) _nodes index1) (Utilities|Array|Get(acopy) _nodes index2)))

(fn FindPath
  (bind _openset (Variables|Default|GetOpenSet))
  (if (Variables|Default|GetUseIndex?)
    (Variables|Default|SetstartNode (Utilities|Array|Get(acopy) (Variables|grid|GetNodes) (Variables|Default|GetStart%20Index)))
    (Variables|Default|SetendNode (Utilities|Array|Get(acopy) (Variables|grid|GetNodes) (Variables|Default|GetEndIndex)))
    (else
      (bind _node (CallFunction|NodefromLoc (Variables|Default|GetStartLoc)))
      (bind _node_2 (CallFunction|NodefromLoc (Variables|Default|GetendLoc)))
      (Variables|Default|SetstartNode _node)
      (Variables|Default|SetendNode _node_2)))
  (Utilities|IsValid (Variables|Default|GetstartNode)
    (:Is%20Valid
      (Utilities|Array|Clear (Variables|Default|GetOpenSet))
      (Utilities|Array|Clear (Variables|Default|GetCloseSet))
      (Utilities|Array|Add (Variables|Default|GetOpenSet) (Variables|Default|GetstartNode))
      (while (!= (Utilities|Array|Length (Variables|Default|GetOpenSet)) 0)
        (Variables|Default|SetcurrentNode (Utilities|Array|Get(acopy) (Variables|Default|GetOpenSet)))
        (for _index (range 0 (- (Utilities|Array|Length _openset) 1))
          (if (Utilities|IsValid (Utilities|Array|Get(acopy) _openset _index))
            (bind _newparam (Default|FCost (Utilities|Array|Get(acopy) _openset _index)))
            (bind _newparam_2 (Default|FCost (Variables|Default|GetcurrentNode)))
            (if (and (<= _newparam _newparam_2) (<= (Variables|/Game/MyContent/BP/AI/BP_Node.BP_Node_C|GetHCost (Utilities|Array|Get(acopy) _openset _index)) (Variables|/Game/MyContent/BP/AI/BP_Node.BP_Node_C|GetHCost (Variables|Default|GetcurrentNode))))
              ;[1 1 1] Set Current Node to be the closest node to the target
              (Variables|Default|SetcurrentNode (Utilities|Array|Get(acopy) (Variables|Default|GetOpenSet) _index)))))
        (Utilities|Array|RemoveItem (Variables|Default|GetOpenSet) (Variables|Default|GetcurrentNode))
        (Utilities|Array|Add (Variables|Default|GetCloseSet) (Variables|Default|GetcurrentNode))
        (if (== (Variables|Default|GetcurrentNode) (Variables|Default|GetendNode))
          ;[1 1 1] ReTracePath
          (bind _output (CallFunction|ReTracePath))
          (return _output)
          (else
            (bind _nodearray (CallFunction|GetNeighbourNodes (Variables|Default|GetcurrentNode)))
            (bind _output_get (Variables|Default|SetNeighbours _nodearray))
            (for _index_2 (range 0 (- (Utilities|Array|Length _output_get) 1))
              (if (and (Utilities|IsValid (Utilities|Array|Get(acopy) (Variables|Default|GetNeighbours) _index_2)) (not (Utilities|Array|ContainsItem (Variables|Default|GetCloseSet) (Utilities|Array|Get(acopy) (Variables|Default|GetNeighbours) _index_2))))
                (bind _distance (CallFunction|GetDistance (Variables|Default|GetcurrentNode) (Utilities|Array|Get(acopy) (Variables|Default|GetNeighbours) _index_2)))
                (Variables|Default|SetnewMovementCostToNeighbour (+ _distance (Variables|/Game/MyContent/BP/AI/BP_Node.BP_Node_C|GetGCost (Variables|Default|GetcurrentNode))))
                (if (or (< (Variables|Default|GetnewMovementCostToNeighbour) (Variables|/Game/MyContent/BP/AI/BP_Node.BP_Node_C|GetGCost (Utilities|Array|Get(acopy) (Variables|Default|GetNeighbours) _index_2))) (not (Utilities|Array|ContainsItem (Variables|Default|GetOpenSet) (Utilities|Array|Get(acopy) (Variables|Default|GetNeighbours) _index_2))))
                  (Variables|/Game/MyContent/BP/AI/BP_Node.BP_Node_C|SetGCost (Utilities|Array|Get(acopy) (Variables|Default|GetNeighbours) _index_2) (Variables|Default|GetnewMovementCostToNeighbour))
                  (bind _distance_2 (CallFunction|GetDistance (Utilities|Array|Get(acopy) (Variables|Default|GetNeighbours) _index_2) (Variables|Default|GetendNode)))
                  (Variables|/Game/MyContent/BP/AI/BP_Node.BP_Node_C|SetHCost (Utilities|Array|Get(acopy) (Variables|Default|GetNeighbours) _index_2) _distance_2)
                  (bind _output_get_2 (Variables|/Game/MyContent/BP/AI/BP_Node.BP_Node_C|SetParentNode (Utilities|Array|Get(acopy) (Variables|Default|GetNeighbours) _index_2) (Variables|Default|GetcurrentNode)))
                  (Rendering|Components|TextRender|SetTextRenderColor (Variables|/Game/MyContent/BP/AI/BP_Node.BP_Node_C|GetNumber _output_get_2) (Variables|Default|GetColor2))
                  (if (not (Utilities|Array|ContainsItem (Variables|Default|GetOpenSet) (Utilities|Array|Get(acopy) (Variables|Default|GetNeighbours) _index_2)))
                    (Utilities|Array|Add (Variables|Default|GetOpenSet) (Utilities|Array|Get(acopy) (Variables|Default|GetNeighbours) _index_2)))))))))
      (bind _location (CallFunction|LocfromNode (Variables|Default|GetstartNode)))
      (return _location))
    (:Is%20Not%20Valid
      (return (Variables|Default|GetStartLoc)))))

(fn GetDistance
  (params (Node1 :type BP%20Node%20Object%20Reference) (Node2 :type BP%20Node%20Object%20Reference))
  (bind _location (CallFunction|LocfromNode Node1))
  (bind _location_2 (CallFunction|LocfromNode Node2))
  (return (Math|Vector|VectorLength (- _location_2 _location))))

(fn ReTracePath
  (if (== (Variables|Default|GetstartNode) (Variables|Default|GetendNode))
    (Utilities|Array|Clear (Variables|Default|GetPath))
    (Variables|Default|SetcurrentNode_forTrace (Variables|Default|GetendNode))
    (while (!= (Variables|Default|GetcurrentNode_forTrace) (Variables|Default|GetstartNode))
      (Utilities|Array|Add (Variables|Default|GetPath) (Variables|Default|GetcurrentNode_forTrace))
      (Variables|Default|SetcurrentNode (Variables|/Game/MyContent/BP/AI/BP_Node.BP_Node_C|GetParentNode (Variables|Default|GetcurrentNode)))
      (bind _arrayelement (Utilities|Array|ReverseforEachLoop (Variables|Default|GetPath))
        (:LoopBody
          (Game|SpawnActorfromClass "/Game/MyContent/BP/AI/BP_NodeIndicator.BP_NodeIndicator_C" (Math|Transform|MakeTransform (Transformation|GetWorldLocation (Variables|/Game/MyContent/BP/AI/BP_Node.BP_Node_C|GetCube _arrayelement)) "0, 0, 0" "1,1,1") "Undefined" 0 0))
        (:Completed
          (return "0, 0, 0"))))))