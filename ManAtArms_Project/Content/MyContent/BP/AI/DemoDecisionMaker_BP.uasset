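; Demo AI actor that follows a MoveArea spline and stops with a "!" text when something is detected below it.
; Each tick, CheckStates evaluates the States data against CurrentState, with Condition mapping condition numbers to functions that switch state.
; Both conditions use a downward debug-drawn line trace, switching to alert on a hit and back on a miss.
; Movement chases a looping, time-driven spline point with speed-capped velocity.
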(event EventBeginPlay
  ;[1 1 1] Initialize
  (Variables|Default|SetCurrentState (Variables|Default|GetInitial%20State)))

(event EventTick
  (params (DeltaSeconds :type Float%20%28single-precision%29))
  ;[0.3711 1 0.7216] On Tick, Do the thing depends on state
  (Class|MyAIBPfunctionLibrary|CheckStates (Variables|Default|GetCurrentState) (Variables|Default|GetStates) self)
  (switch int (Variables|Default|GetCurrentState)
    (:0
      ;;[1 1 1] State_0
      (Utilities|IsValid (Variables|Default|GetMoveArea)
        (:Is%20Valid
          (CallFunction|Move DeltaSeconds)
          (Rendering|Components|TextRender|SetText (Variables|Default|GetTextRender) (Utilities|Text|ToText(String) (Utilities|String|Append "" ""))))))
    (:1
      ;;[1 1 1] State_1
      (Rendering|Components|TextRender|SetText (Variables|Default|GetTextRender) (Utilities|Text|ToText(String) (Utilities|String|Append "!" ""))))))

(fn ConstructionScript)

(fn Condition1
  (bind _returnvalue (Transformation|GetActorLocation))
  (bind (_x _y _z) (Math|Vector|BreakVector _returnvalue))
  (bind _returnvalue_2 (Collision|LineTraceByChannel (Transformation|GetActorLocation) (Math|Vector|MakeVector _x _y (- _z (Variables|Default|GetDetectionLength))) "TraceTypeQuery1" false 0 "ForOneFrame"))
  (return _returnvalue_2 1))

(fn Condition2
  (bind _returnvalue (Transformation|GetActorLocation))
  (bind (_x _y _z) (Math|Vector|BreakVector _returnvalue))
  (bind _returnvalue_2 (Collision|LineTraceByChannel (Transformation|GetActorLocation) (Math|Vector|MakeVector _x _y (- _z (Variables|Default|GetDetectionLength))) "TraceTypeQuery1" false 0 "ForOneFrame"))
  (return (not _returnvalue_2) 0))

(fn CheckStates
  (params (CurrentState_in :type Integer))
  (Class|MyAIBPfunctionLibrary|CheckStates CurrentState_in (Variables|Default|GetStates) self))

(fn Condition
  (params (condition :type String))
  (switch int (Math|Conversions|ToInteger(Byte) condition)
    (:1
      (bind (_go _state) (CallFunction|Condition1))
      (if _go
        (Variables|Default|SetCurrentState _state)))
    (:2
      (bind (_go_2 _state_2) (CallFunction|Condition2))
      (if _go_2
        (Variables|Default|SetCurrentState _state_2)))))

(fn Move
  (params (timerTick :type Float%20%28single-precision%29))
  (bind _movearea (Variables|Default|GetMoveArea))
  (bind _spline (Variables|/Game/MyContent/BP/AI/MoveArea.MoveArea_C|GetSpline _movearea))
  (if (> (* (Variables|Default|GetTimer) (Variables|Default|GetSpeed)) (Spline|GetSplineLength _spline))
    (Variables|Default|SetTimer 0.0)
    (else
      (Variables|Default|SetTimer (+ timerTick (Variables|Default|GetTimer)))
      (bind _output_get (Variables|Default|Setvelocity (/ (- (Spline|GetLocationatDistanceAlongSpline _spline (* (Variables|Default|GetTimer) (Variables|Default|GetSpeed)) "World") (Transformation|GetActorLocation)) (Variables|Default|GetTimeToTarget))))
      (if (> (Math|Vector|VectorLength _output_get) (Variables|Default|GetMaxSpeed))
        (Variables|Default|Setvelocity (* (Math|Vector|Normalize (Variables|Default|Getvelocity)) (Variables|Default|GetMaxSpeed))))
      (Transformation|SetActorLocationAndRotation (+ (Transformation|GetActorLocation) (* (Variables|Default|Getvelocity) timerTick)) "0, 0, 0"))))