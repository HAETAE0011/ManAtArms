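; BP_Node is a grid node actor for AI pathfinding, holding grid coordinates, a cached world location and G/H costs.
; FCost returns GCost plus HCost in A* style, and SetGridValues stores the node's X and Y position.
; The construction script caches the actor location.
; Shortly after BeginPlay, two text elements display the node's number and one of two availability labels based on the AS flag.
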(event EventBeginPlay
  (bind _available (Variables|Default|GetAvailable))
  (Utilities|FlowControl|Delay 0.2)
  (Rendering|Components|TextRender|SetText (Variables|Default|GetNumber) (Utilities|Text|ToText(Integer) (Variables|Default|Getnum)))
  (if (Variables|Default|GetAS)
    (Rendering|Components|TextRender|SetText _available (Variables|Default|Gettext1))
    (else
      (Rendering|Components|TextRender|SetText _available (Variables|Default|Gettext2)))))

(event Collision|EventActorBeginOverlap
  (params (OtherActor :type Actor%20Object%20Reference)))

(event EventTick
  (params (DeltaSeconds :type Float%20%28single-precision%29)))

(fn ConstructionScript
  (Variables|Default|SetLocation (Transformation|GetActorLocation)))

(fn FCost
  (return (+ (Variables|Default|GetGCost) (Variables|Default|GetHCost))))

(fn SetGridValues
  (params (X :type Integer) (Y :type Integer))
  (Variables|Default|SetGrid_X X)
  (Variables|Default|SetGrid_Y Y))