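; BP_SplineOutliner lines an editable spline with deformed meshes at construction time.
; The construction script resamples the spline at a fixed segment length into a temporary spline, which it destroys after building a spline mesh per segment.
; Segments use one mesh or random picks from a list via a seeded stream, reseeded by the Refresh toggle.
; An uncalled SplineMeshCreation function offers a start, middle and end mesh variant.
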(event EventBeginPlay)

(event Collision|EventActorBeginOverlap
  (params (OtherActor :type Actor%20Object%20Reference)))

(event EventTick
  (params (DeltaSeconds :type Float%20%28single-precision%29)))

(fn ConstructionScript
  (bind _spline (Variables|Default|GetSpline))
  (bind _mesh_list (Variables|Meshes|GetMesh%20List))
  (bind _lengthpereachspline (Variables|OnlyOneSpline|GetLengthPerEachSpline))
  ;[1 1 1] Refresh function
  (if (Variables|Base|GetRefresh)
    (Class|KismetMathLibrary|SeedRandomStream (Variables|Default|GetStream))
    (Variables|Base|SetRefresh false))
  ;[1 1 1] Only one Spline
  (bind _returnvalue (AddComponent|AddSplineComponent false))
  (Spline|ClearSplinePoints _returnvalue true)
  ;;[1 1 1] Regulate the distance between points in spline
  (for _index (range 0 (Math|Float|Truncate (/ (- (Spline|GetDistanceAlongSplineatSplinePoint _spline (- (Spline|GetNumberOfSplinePoints _spline) 1)) (Spline|GetDistanceAlongSplineatSplinePoint _spline 0)) _lengthpereachspline)))
    (Spline|AddSplinePoint _returnvalue (Spline|GetLocationatDistanceAlongSpline _spline (* _index _lengthpereachspline) "World") "World" true))
  ;;[0.3098 0.2078 1] Create Spline Mesh
  (for _index_2 (range 0 (- (Spline|GetNumberOfSplinePoints _returnvalue) 2))
    (bind _returnvalue_2 (AddComponent|AddSplineMeshComponent false))
    (SplineMesh|SetForwardAxis _returnvalue_2 (Variables|Default|GetForwardAxis) true)
    (if (Variables|Meshes|GetMultiple%20Mesh?)
      (Components|StaticMesh|SetStaticMesh _returnvalue_2 (Utilities|Array|Get(acopy) _mesh_list (Math|Random|RandomIntegerinRangefromStream 0 (- (Utilities|Array|Length _mesh_list) 1) (Variables|Default|GetStream))))
      (else
        (Components|StaticMesh|SetStaticMesh _returnvalue_2 (Variables|Meshes|GetMesh))))
    (SplineMesh|SetStartandEnd _returnvalue_2 (Spline|GetLocationatSplinePoint _returnvalue _index_2 "Local") (Spline|GetTangentatSplinePoint _returnvalue _index_2 "Local") (Spline|GetLocationatSplinePoint _returnvalue (+ _index_2 1) "Local") (Spline|GetTangentatSplinePoint _returnvalue (+ _index_2 1) "Local") true :!class /Script/Engine.SplineMeshComponent))
  ;;[0.25 0.03448 0.2014] At the end, Clear the splines/points created
  (Spline|ClearSplinePoints _returnvalue true)
  (Components|DestroyComponent _returnvalue))

(fn SplineMeshCreation
  (params (Spline :type Spline%20Component%20Object%20Reference) (Start :type Static%20Mesh%20Object%20Reference) (Middle :type Static%20Mesh%20Object%20Reference) (End :type Static%20Mesh%20Object%20Reference))
  (bind _returnvalue (Spline|GetNumberOfSplinePoints Spline))
  (bind _returnvalue_2 (- _returnvalue 2))
  ;[1 1 1] Spline Mesh
  (for _index (range 0 _returnvalue_2)
    (bind _returnvalue_3 (AddComponent|AddSplineMeshComponent false))
    (if (== _index 0)
      ;;[1 0.4688 0.4688] Three Meshes- start, middle, end
      (Components|StaticMesh|SetStaticMesh _returnvalue_3 Start)
      (elif (== _returnvalue_2 _index)
        (Components|StaticMesh|SetStaticMesh _returnvalue_3 End)
        (else
          (Components|StaticMesh|SetStaticMesh _returnvalue_3 Middle))))
    (SplineMesh|SetStartandEnd _returnvalue_3 (Spline|GetLocationatSplinePoint Spline _index "Local") (Spline|GetTangentatSplinePoint Spline _index "Local") (Spline|GetLocationatSplinePoint Spline (+ _index 1) "Local") (Spline|GetTangentatSplinePoint Spline (+ _index 1) "Local") true :!class /Script/Engine.SplineMeshComponent)))