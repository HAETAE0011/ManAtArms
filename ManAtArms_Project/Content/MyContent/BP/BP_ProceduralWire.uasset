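; Procedural wire builder that generates spline-mesh wires along an editable guide spline in the construction script.
; SplineType picks the layout: offset copies, surface-offset strands with optional instanced sub-meshes, random branches off a core, or one evenly re-spaced spline.
; Each builds temporary splines using a seeded random stream and offset curve for variation.
; SplineMeshCreation or inline logic lays start, middle and end meshes per segment.
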(event EventBeginPlay)

(event Collision|EventActorBeginOverlap
  (params (OtherActor :type Actor%20Object%20Reference)))

(event EventTick
  (params (DeltaSeconds :type Float%20%28single-precision%29)))

(fn ConstructionScript
  (bind _spline (Variables|Default|GetSpline))
  (bind _arrow (Variables|Default|GetArrow))
  (bind _spline_2 (Variables|Default|GetSpline))
  (bind _spline_3 (Variables|Default|GetSpline))
  (bind _distancebetweensubmeshs (Variables|Surface|GetDistanceBetweenSubmeshs))
  (bind _spline_4 (Variables|Default|GetSpline))
  (bind _offsetminvalue (Variables|Values|GetOffsetMinValue))
  (bind _offsetmaxvalue (Variables|Values|GetOffsetMaxValue))
  (bind _branch_end_offset (Variables|Branch|GetBranch%20end%20offset))
  (bind _randomseed (Variables|Default|GetRandomSeed))
  (bind _lengthpereachspline (Variables|OnlyOneSpline|GetLengthPerEachSpline))
  (bind _returnvalue (Spline|GetNumberOfSplinePoints _spline_4))
  (bind _returnvalue_2 (Spline|GetNumberOfSplinePoints _spline_2))
  (bind _returnvalue_3 (Spline|GetDistanceAlongSplineatSplinePoint _spline_2 1))
  (bind _returnvalue_4 (Math|Random|RandomIntegerinRangefromStream 0 _branch_end_offset _randomseed))
  (bind _returnvalue_5 (Spline|GetNumberOfSplinePoints _spline_3))
  (bind _returnvalue_6 (- _returnvalue_5 1))
  (bind _returnvalue_7 (- _returnvalue 1))
  (bind _returnvalue_8 (- _returnvalue_2 1))
  (bind _returnvalue_9 (- _returnvalue_8 2))
  (bind _returnvalue_10 (- _returnvalue_7 _returnvalue_4))
  (bind _returnvalue_11 (Spline|GetDistanceAlongSplineatSplinePoint _spline_2 _returnvalue_9))
  (Components|StaticMesh|SetStaticMesh (Variables|Default|GetSubMesh) (Variables|Meshes|GetMeshesOnSpline))
  ;[1 1 1] Refresh function
  (if (Variables|Base|GetRefresh)
    (Variables|Base|SetRefresh false)
    (Class|KismetMathLibrary|SeedRandomStream (Variables|Default|GetRandomSeed)))
  (switch Utilities|FlowControl|Switch|SwitchonSplineTypes (Variables|Base|GetSplineType)
    (:NewEnumerator0
      ;[1 1 1] Basic Following Spline
      (for _index (range 1 (Variables|Base|GetNumberOfWires))
        ;;[0.06994 1 0.7583] Create Spline around original Spline
        (bind _returnvalue_12 (AddComponent|AddSplineComponent false))
        (Spline|ClearSplinePoints _returnvalue_12 true)
        (for _index_2 (range 0 _returnvalue_6)
          (Spline|AddSplinePoint _returnvalue_12 (+ (Spline|GetLocationatSplinePoint _spline_3 _index_2 "World") (* (* (Math|Vector|MakeVector (Math|Random|RandomFloatinRangefromStream _offsetminvalue _offsetmaxvalue (Variables|Default|GetRandomSeed)) (Math|Random|RandomFloatinRangefromStream _offsetminvalue _offsetmaxvalue (Variables|Default|GetRandomSeed)) (Math|Random|RandomFloatinRangefromStream _offsetminvalue _offsetmaxvalue (Variables|Default|GetRandomSeed))) (Math|Curves|GetFloatValue (Variables|Curve|GetLocationOffsetCurve) (/ (Math|Conversions|ToFloat(Integer) _index_2) (Math|Conversions|ToFloat(Integer) _returnvalue_6)))) (Variables|BasicFollow|GetBasicOffsetAxis))) "World" true))
        ;;[0.3098 0.2078 1] Create Spline Mesh
        (CallFunction|SplineMeshCreation _returnvalue_12 (Variables|Meshes|GetMesh_Start) (Variables|Meshes|GetMesh_Middle) (Variables|Meshes|GetMesh_End))))
    (:NewEnumerator1
      ;[1 1 1] On Surface
      (for _index_3 (range 1 (Variables|Base|GetNumberOfWires))
        (bind _returnvalue_13 (AddComponent|AddSplineComponent false))
        (Spline|ClearSplinePoints _returnvalue_13 true)
        (for _index_4 (range 0 _returnvalue_10)
          (if (== _index_4 0)
            ;;[1 1 1] initial point of branch
            (Spline|AddSplinePoint _returnvalue_13 (+ (Spline|GetLocationatSplinePoint _spline_4 _index_4 "Local") (* (Variables|Surface|GetSurfaceOffsetAxis) (+ (Math|Random|RandomFloatinRangefromStream (Variables|Values|GetOffsetMinValue) (Variables|Values|GetOffsetMaxValue) (Variables|Default|GetRandomSeed)) (Math|Curves|GetFloatValue (Variables|Curve|GetLocationOffsetCurve) (/ (Math|Conversions|ToFloat(Integer) _returnvalue_10) (Math|Conversions|ToFloat(Integer) _index_4)))))) "Local" true)
            (else
              ;;[1 1 1] The rest of points
              (Spline|AddSplinePoint _returnvalue_13 (+ (Spline|GetLocationatSplinePoint _returnvalue_13 (- _index_4 1) "Local") (+ (- (Spline|GetLocationatSplinePoint _spline_4 _index_4 "Local") (Spline|GetLocationatSplinePoint _spline_4 (- _index_4 1) "Local")) (* (Variables|Surface|GetSurfaceOffsetAxis) (Math|Random|RandomFloatinRangefromStream (Variables|Values|GetOffsetMinValue_2) (Variables|Values|GetOffsetMaxValue_2) (Variables|Default|GetRandomSeed))))) "Local" true))))
        (Utilities|FlowControl|Sequence
          (:then_0
            (if (Variables|Base|GetShowSplineMesh)
              ;;[0.3098 0.2078 1] Create Spline Mesh
              (CallFunction|SplineMeshCreation _returnvalue_13 (Variables|Meshes|GetMesh_Start) (Variables|Meshes|GetMesh_End) (Variables|Meshes|GetMesh_Middle))))
          (:then_1
            ;;[0.4062 1 0.4841] Sub Meshes
            (if (Variables|Base|GetShowSubMesh)
              (for _index_5 (range 0 (Math|Float|Truncate (/ (Spline|GetSplineLength _returnvalue_13) _distancebetweensubmeshs)))
                (Class|InstancedStaticMeshComponent|AddInstanceWorldSpace (Variables|Default|GetSubMesh) (Math|Transform|MakeTransform (Spline|GetLocationatDistanceAlongSpline _returnvalue_13 (* _index_5 _distancebetweensubmeshs) "World") (Math|Rotator|MakeRotationfromAxes (Math|Vector|GetForwardVector (Math|Conversions|RotationFromXVector (.Tangent (Spline|GetLocationandTangentatSplinePoint _returnvalue_13 _index_5 "World")))) (- (Math|Vector|GetRightVector _arrow) (- (Math|Vector|GetRightVector (Variables|Default|GetArrow)) (Class|SplineComponent|GetRightVectoratSplinePoint _returnvalue_13 _index_5 "World"))) (Math|Vector|GetForwardVector _arrow)) (Math|Vector|MakeVector (* (Math|Curves|GetFloatValue (Variables|Curve|GetSizeCurve) (/ (Math|Conversions|ToFloat(Integer) _index_5) (Math|Conversions|ToFloat(Integer) (Math|Float|Truncate (/ (Spline|GetSplineLength _returnvalue_13) _distancebetweensubmeshs))))) (Math|Random|RandomFloatinRangefromStream 1.5 3.5 (Variables|Default|GetRandomSeed))) (* (Math|Curves|GetFloatValue (Variables|Curve|GetSizeCurve) (/ (Math|Conversions|ToFloat(Integer) _index_5) (Math|Conversions|ToFloat(Integer) (Math|Float|Truncate (/ (Spline|GetSplineLength _returnvalue_13) _distancebetweensubmeshs))))) (Math|Random|RandomFloatinRangefromStream 1.5 3.5 (Variables|Default|GetRandomSeed))) (* (Math|Curves|GetFloatValue (Variables|Curve|GetSizeCurve) (/ (Math|Conversions|ToFloat(Integer) _index_5) (Math|Conversions|ToFloat(Integer) (Math|Float|Truncate (/ (Spline|GetSplineLength _returnvalue_13) _distancebetweensubmeshs))))) (Math|Random|RandomFloatinRangefromStream 1.5 3.5 (Variables|Default|GetRandomSeed)))))))
              ;;;[0.25 0.03448 0.2014] At the end, Clear the splines/points created
              (Spline|ClearSplinePoints _returnvalue_13 true)
              (Components|DestroyComponent _returnvalue_13)))))
      ;;[0.25 0.03448 0.2014] At the end, Clear the splines/points created
      (Spline|ClearSplinePoints _returnvalue_13 true)
      (Components|DestroyComponent _returnvalue_13))
    (:NewEnumerator3
      ;[1 1 1] Branches
      ;;[0.06994 1 0.7583] Create Spline around original Spline
      (bind _returnvalue_14 (AddComponent|AddSplineComponent false))
      (Spline|ClearSplinePoints _returnvalue_14 true)
      (for _index_6 (range 0 (- (Spline|GetNumberOfSplinePoints _spline) 1))
        (Spline|AddSplinePoint _returnvalue_14 (+ (Spline|GetLocationatSplinePoint _spline _index_6 "Local") "0, 0, 0") "Local" true))
      (for _index_7 (range 1 (Variables|Base|GetNumberOfWires))
        ;;[0.3447 0.3333 1] finds where to start the branch
        (bind _index_8 (Utilities|FlowControl|ForLoopwithBreak 0 (- (Spline|GetNumberOfSplinePoints _returnvalue_14) (Variables|Branch|GetSubSplineLength)) :!label _label)
          (:LoopBody
            (if (> (Spline|GetDistanceAlongSplineatSplinePoint _returnvalue_14 _index_8) (Math|Random|RandomFloatinRangefromStream (Variables|Branch|GetbranchStartOffset) (Spline|GetDistanceAlongSplineatSplinePoint _returnvalue_14 (- (Spline|GetNumberOfSplinePoints _returnvalue_14) (Variables|Branch|GetSubSplineLength))) (Variables|Default|GetRandomSeed)))
              (Variables|Default|SetTreeStartOffset_temp _index_8)
              (goto _label Break)))
          (:Completed
            ;;[0 1 0.1234] Set which direction the branches will go out
            (Variables|Default|SetTempVector (* (Variables|Branch|GetBranchOffsetAxis) (Math|Random|RandomFloatinRangefromStream (Variables|Values|GetOffsetMinValue) (Variables|Values|GetOffsetMaxValue) (Variables|Default|GetRandomSeed))))
            ;;[1 1 1] Spline point creation
            (bind _returnvalue_15 (AddComponent|AddSplineComponent false))
            (Spline|ClearSplinePoints _returnvalue_15 true)
            (for _index_9 (range (Variables|Default|GetTreeStartOffset_temp) (+ (Variables|Default|GetTreeStartOffset_temp) (Variables|Branch|GetSubSplineLength)))
              (if (== (Variables|Default|GetTreeStartOffset_temp) _index_9)
                ;;;[1 0.2703 0.2603] Initial point of branch should start from core spline
                (Spline|AddSplinePoint _returnvalue_15 (Spline|GetLocationatSplinePoint _returnvalue_14 _index_9 "Local") "Local" true)
                (else
                  (Spline|AddSplinePoint _returnvalue_15 (+ (Spline|GetLocationatSplinePoint _returnvalue_14 _index_9 "Local") (Variables|Default|GetTempVector)) "Local" true))))
            (if (Variables|Base|GetShowSplineMesh)
              ;;[0.3098 0.2078 1] Create Spline Mesh
              (CallFunction|SplineMeshCreation _returnvalue_15 (Variables|Meshes|GetSubMesh_Start) (Variables|Meshes|GetSubMesh_Middle) (Variables|Meshes|GetSubMesh_End))
              ;;[0.25 0.03448 0.2014] At the end, Clear the splines/points created
              (Spline|ClearSplinePoints _returnvalue_15 true)
              (Components|DestroyComponent _returnvalue_15)))))
      (if (Variables|Base|GetShowSplineMesh)
        ;;[0.3098 0.2078 1] Create Spline Mesh
        (CallFunction|SplineMeshCreation _returnvalue_14 (Variables|Meshes|GetMesh_Start) (Variables|Meshes|GetMesh_Middle) (Variables|Meshes|GetMesh_End))
        ;;[0.25 0.03448 0.2014] At the end, Clear the splines/points created
        (Spline|ClearSplinePoints _returnvalue_14 true)
        (Components|DestroyComponent _returnvalue_14)))
    (:NewEnumerator2
      ;[1 1 1] Only one Spline
      (bind _returnvalue_16 (AddComponent|AddSplineComponent false))
      (Spline|ClearSplinePoints _returnvalue_16 true)
      (Variables|Default|SetDistanceBetweenSubmeshsChecker 0.0)
      (for _index_10 (range 0 _returnvalue_8)
        ;;[1 1 1] Initial 2 point
        (if (<= _index_10 1)
          (Spline|AddSplinePoint _returnvalue_16 (Spline|GetLocationatSplinePoint _spline_2 _index_10 "World") "World" true)))
      ;;[1 1 1] Regulate the distance between points in spline
      (for _index_11 (range 0 (Math|Float|Truncate (- _returnvalue_11 _returnvalue_3)))
        (if (or (<= _returnvalue_11 (Variables|Default|GetDistanceBetweenSubmeshsChecker)) (>= _returnvalue_3 (Variables|Default|GetDistanceBetweenSubmeshsChecker)))
          _
          (else
            (Spline|AddSplinePoint _returnvalue_16 (Spline|GetLocationatDistanceAlongSpline _spline_2 (* _index_11 _lengthpereachspline) "World") "World" true)))
        (Variables|Default|SetDistanceBetweenSubmeshsChecker (+ (Variables|Default|GetDistanceBetweenSubmeshsChecker) _lengthpereachspline)))
      ;;[1 1 1] Last 2 point
      (for _index_12 (range 0 _returnvalue_8)
        (if (>= _index_12 (- _returnvalue_8 2))
          (Spline|AddSplinePoint _returnvalue_16 (Spline|GetLocationatSplinePoint _spline_2 _index_12 "World") "World" true)))
      ;;[0.3098 0.2078 1] Create Spline Mesh
      (for _index_13 (range 0 (- (Spline|GetNumberOfSplinePoints _returnvalue_16) 2))
        (bind _returnvalue_17 (AddComponent|AddSplineMeshComponent false))
        (if (== _index_13 0)
          ;;;[1 0.4688 0.4688] Three Meshes- start, middle, end
          (Components|StaticMesh|SetStaticMesh _returnvalue_17 (Variables|Meshes|GetMesh_Start))
          (elif (== (- (Spline|GetNumberOfSplinePoints _returnvalue_16) 2) _index_13)
            (Components|StaticMesh|SetStaticMesh _returnvalue_17 (Variables|Meshes|GetMesh_End))
            (else
              (Components|StaticMesh|SetStaticMesh _returnvalue_17 (Variables|Meshes|GetMesh_Middle)))))
        (SplineMesh|SetStartandEnd _returnvalue_17 (Spline|GetLocationatSplinePoint _returnvalue_16 _index_13 "Local") (Spline|GetTangentatSplinePoint _returnvalue_16 _index_13 "Local") (Spline|GetLocationatSplinePoint _returnvalue_16 (+ _index_13 1) "Local") (Spline|GetTangentatSplinePoint _returnvalue_16 (+ _index_13 1) "Local") true :!class /Script/Engine.SplineMeshComponent))
      ;;[0.25 0.03448 0.2014] At the end, Clear the splines/points created
      (Spline|ClearSplinePoints _returnvalue_16 true)
      (Components|DestroyComponent _returnvalue_16))))

(fn SplineMeshCreation
  (params (Spline :type Spline%20Component%20Object%20Reference) (Start :type Static%20Mesh%20Object%20Reference) (Middle :type Static%20Mesh%20Object%20Reference) (End :type Static%20Mesh%20Object%20Reference))
  (bind _returnvalue (Spline|GetNumberOfSplinePoints Spline))
  (bind _returnvalue_2 (- _returnvalue 2))
  ;[1 1 1] Spline Mesh
  (for _index (range 0 _returnvalue_2)
    (bind _returnvalue_3 (AddComponent|AddSplineMeshComponent false))
    (if (== _index 0)
      ;;[1 0.4688 0.4688] Three Meshes- start, middle, end
      (Components|StaticMesh|SetStaticMesh _returnvalue_3 Start)
      (elif (== _returnvalue_2 _index)
        (Components|StaticMesh|SetStaticMesh _returnvalue_3 End)
        (else
          (Components|StaticMesh|SetStaticMesh _returnvalue_3 Middle))))
    (SplineMesh|SetStartandEnd _returnvalue_3 (Spline|GetLocationatSplinePoint Spline _index "Local") (Spline|GetTangentatSplinePoint Spline _index "Local") (Spline|GetLocationatSplinePoint Spline (+ _index 1) "Local") (Spline|GetTangentatSplinePoint Spline (+ _index 1) "Local") true :!class /Script/Engine.SplineMeshComponent)))