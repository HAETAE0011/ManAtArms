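; BP_GroupMovementMaster produces a wandering CurrentTarget location, apparently to steer group movement.
; On Tick, a timer periodically picks a random NextTarget inside MovableArea, snapping Target to it the first time.
; Between picks, Target moves toward NextTarget at constant speed.
; A debug-drawn visibility trace from the actor to Target updates CurrentTarget only when nothing blocks it.
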(event EventTick
  (params (DeltaSeconds :type Float%20%28single-precision%29))
  ;[1 1 1] Timer
  (if (> (Variables|Default|GetTimer) (Variables|Default|GetTimeToSetNewTarget))
    (Variables|Default|SetTimer 0.0)
    ;[1 1 1] if timer is over
    (bind _randompoint (Default|GetRandomPoint (Variables|Default|GetMovableArea)))
    (Variables|Default|SetnextTarget _randompoint)
    ;[1 1 1] Initialize Target
    (Utilities|FlowControl|DoOnce false
      (:Completed
        (Variables|Default|Settarget (Variables|Default|GetnextTarget))))
    (else
      (Variables|Default|SetTimer (+ DeltaSeconds (Variables|Default|GetTimer)))
      ;[1 1 1] Update target location
      (bind _output_get (Variables|Default|Settarget (+ (Variables|Default|Gettarget) (* (Math|Vector|Normalize (- (Variables|Default|GetnextTarget) (Variables|Default|Gettarget))) (* DeltaSeconds (Variables|Default|GetSpeedBetweenTnT))))))
      (bind _returnvalue (Collision|LineTraceByChannel (Transformation|GetActorLocation) _output_get "TraceTypeQuery1" true 0 "ForOneFrame"))
      (if (not _returnvalue)
        (Variables|Default|SetCurrentTarget (Variables|Default|Gettarget))))))

(fn ConstructionScript)