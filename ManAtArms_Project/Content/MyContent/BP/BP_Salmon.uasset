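; BP_Salmon is a fish actor that swims between random points in a MovableArea using Kinematic Arrive steering on Tick.
; It moves toward its Target at speed scaled by TimeToTarget, capped at MaxSpeed, and faces its velocity.
; Within Radius it picks a new point, sometimes pausing for FoodTime first.
; In GroupMovement mode it instead follows GroupMaster's target, randomly offset on arrival.
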(event EventTick
  (params (DeltaSeconds :type Float%20%28single-precision%29))
  (bind _groupmaster (Variables|Default|GetGroupMaster))
  (bind _groupmaster_2 (Variables|Default|GetGroupMaster))
  (bind _target (Variables|/Game/MyContent/BP/BP_GroupMovementMaster.BP_GroupMovementMaster_C|Gettarget _groupmaster))
  ;[1 1 1] KinematicArrive Mechanic
  (|CallParentFunction DeltaSeconds)
  ;;[1 0.4635 0.4635] Checks if Movable Area is vaild
  (if (Utilities|IsValid (Variables|Default|GetMovableArea))
    ;;[0.3585 1 0.3841] when the Target is not 0,0,0 (default)
    (if (Math|Vector|NotEqual(Vector) (Variables|Default|GetTarget) "0, 0, 0" 0.0001)
      ;;[0.1226 0.2971 0.3229] Checks if the object is far enough to the Target location
      (if (> (Math|Vector|VectorLength (- (Variables|Default|GetTarget) (Transformation|GetActorLocation))) (Variables|Default|GetRadius))
        ;;[0.3997 0.6132 1] Set Velocity
        (bind _output_get (Variables|Default|Setvelocity (/ (- (Variables|Default|GetTarget) (Transformation|GetActorLocation)) (Variables|Default|GetTimeToTarget))))
        ;;[0.6895 0.2794 1] if velocity length > maxSpeed, then clip to max speed
        (if (> (Math|Vector|VectorLength _output_get) (Variables|Default|GetMaxSpeed))
          (Variables|Default|Setvelocity (* (Math|Vector|Normalize (Variables|Default|Getvelocity)) (Variables|Default|GetMaxSpeed))))
        (Transformation|SetActorLocationAndRotation (+ (Transformation|GetActorLocation) (* (Variables|Default|Getvelocity) DeltaSeconds)) (Math|Rotator|MakeRotfromX (Variables|Default|Getvelocity)))
        (else
          ;;[1 0.5566 0.4463] Set random Target location to move
          (if (Variables|Default|GetGroupMovement?)
            (Utilities|IsValid _groupmaster_2
              (:Is%20Valid
                (bind _outputvector (CallFunction|GetAroundVector (Variables|/Game/MyContent/BP/BP_GroupMovementMaster.BP_GroupMovementMaster_C|Gettarget _groupmaster_2)))
                (Variables|Default|SetTarget _outputvector)))
            (else
              (Utilities|FlowControl|DoOnce false :!label _label
                (:Completed
                  (if (> (Math|Random|RandomFloatinRangefromStream 0.0 1.0 (Variables|Default|GetStream4)) 0.3)
                    (CallFunction|SetRandomTarget)
                    (goto _label Reset)
                    (else
                      (Utilities|FlowControl|Delay (Variables|Default|GetFoodTime!))
                      (CallFunction|SetRandomTarget)
                      (Class|KismetMathLibrary|SeedRandomStream (Variables|Default|GetStream4))
                      (goto _label Reset)))))))))
      (else
        ;;[0.2081 0.5332 1] Set random Target location to move
        (if (Variables|Default|GetGroupMovement?)
          (Utilities|IsValid _groupmaster
            (:Is%20Valid
              (CallFunction|GetAroundVector _target)
              (Variables|Default|SetTarget _target)))
          (else
            (CallFunction|SetRandomTarget)))))))

(fn ConstructionScript
  (|CallParentFunction))

(fn SetRandomTarget
  (bind _randompoint (Default|GetRandomPoint (Variables|Default|GetMovableArea)))
  (Variables|Default|SetTarget _randompoint))

(fn GetAroundVector
  (params (InputVector :type Vector))
  (bind _randomvectoroffset (Variables|Default|GetRandomVectorOffset))
  (Class|KismetMathLibrary|SeedRandomStream (Variables|Default|GetStream1))
  (Class|KismetMathLibrary|SeedRandomStream (Variables|Default|GetStream2))
  (Class|KismetMathLibrary|SeedRandomStream (Variables|Default|GetStream3))
  (return (+ InputVector (Math|Vector|MakeVector (Math|Random|RandomFloatinRangefromStream (* _randomvectoroffset -1.0) 0.0 (Variables|Default|GetStream1)) (Math|Random|RandomFloatinRangefromStream (* _randomvectoroffset -1.0) 0.0 (Variables|Default|GetStream2)) (Math|Random|RandomFloatinRangefromStream (* _randomvectoroffset -1.0) 0.0 (Variables|Default|GetStream3))))))