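; BP_TestEnemy is a test enemy actor that shows its health on a TextRender component.
; BeginPlay writes the starting Health as an "HP:" label.
; The GetDamage function subtracts the given damage from Health, refreshes the label, and destroys the actor once Health is zero or below.
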(event EventBeginPlay
  (Rendering|Components|TextRender|SetText (Variables|Default|GetTextRender) (Utilities|Text|ToText(String) (Utilities|String|Append "HP:" (Utilities|String|ToString(Float) (Variables|Default|GetHealth))))))

(fn ConstructionScript)

(fn GetDamage
  (params (Damage :type Float%20%28single-precision%29))
  (Variables|Default|SetHealth (- (Variables|Default|GetHealth) Damage))
  (Rendering|Components|TextRender|SetText (Variables|Default|GetTextRender) (Utilities|Text|ToText(String) (Utilities|String|Append "HP:" (Utilities|String|ToString(Float) (Variables|Default|GetHealth)))))
  (if (<= (Variables|Default|GetHealth) 0.0)
    (Actor|DestroyActor)))