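; BP_BuildingMaker is a procedural building actor that assembles walls and pillars from instanced static meshes in its Construction Script.
; MakeFloor lays four walls per floor, using one float curve per side to pick each segment's mesh, falling back to the last valid curve.
; MakeWall adds random tilt, while optional branches place corner pillars, horizontal beams and interior vertical pillar grids.
; Roof generation is unfinished and produces nothing.
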(event EventBeginPlay)

(event Collision|EventActorBeginOverlap
  (params (OtherActor :type Actor%20Object%20Reference)))

(event EventTick
  (params (DeltaSeconds :type Float%20%28single-precision%29)))

(fn ConstructionScript
  (bind _wallmeshes (Variables|Mesh|GetWallMeshes))
  (bind _meshes_instances (Variables|Mesh|GetMeshes_instances))
  (bind _numberoffloors (Variables|Base|GetNumberOfFloors))
  (bind _outerpillar (Variables|Default|GetOuterPillar))
  (bind _pillar_horizontal (Variables|Default|GetPillar_horizontal))
  (bind _height (Variables|Base|GetHeight))
  (bind _numberoffloors_2 (Variables|Base|GetNumberOfFloors))
  (bind _width (Variables|Base|GetWidth))
  (bind _numberofhorizontalpillars (Variables|Base|GetNumberOfHorizontalPillars))
  (bind _horizontalpillarlength (Variables|Base|GetHorizontalPillarLength))
  (bind _returnvalue (- _numberoffloors 1))
  (bind _returnvalue_2 (/ _numberofhorizontalpillars 2))
  (bind _returnvalue_3 (* _numberoffloors_2 _height))
  (bind _returnvalue_4 (/ _width _horizontalpillarlength))
  (bind _returnvalue_5 (- _returnvalue_3 15.0))
  ;[1 1 1] Initialize Instanced Static Meshes
  ;;[1 0.3958 0.3958] Initialize ISM Arrays
  (Utilities|Array|Clear _meshes_instances)
  (for _index (range 0 (Utilities|Array|LastIndex _wallmeshes))
    (bind _returnvalue_6 (AddComponent|AddInstancedStaticMeshComponent false))
    (Components|StaticMesh|SetStaticMesh _returnvalue_6 (Utilities|Array|Get(acopy) _wallmeshes _index))
    (Utilities|Array|Add _meshes_instances _returnvalue_6))
  (Components|StaticMesh|SetStaticMesh (Variables|Default|GetOuterPillar) (Variables|Mesh|GetOuterPillarMesh))
  (Components|StaticMesh|SetStaticMesh (Variables|Default|GetPillar_horizontal) (Variables|Mesh|GetHorizontalPillarMesh))
  (Components|StaticMesh|SetStaticMesh (Variables|Default|GetPillar_Vertical) (Variables|Mesh|GetVerticalPillarMesh))
  ;[1 1 1] Refresh function
  (if (Variables|Base|Getrefresh)
    (Variables|Base|Setrefresh false)
    (else
      (Utilities|FlowControl|DoOnce false
        (:Completed
          _))))
  ;[1 1 1] Setting the size of curve array
  (Utilities|Array|Resize (Variables|Curve|GetWallFormingCurves) (* (Variables|Base|GetNumberOfFloors) 4))
  ;[1 1 1] Make Building
  (Utilities|FlowControl|Sequence
    (:then_0
      (for _index_2 (range 0 _returnvalue)
        ;;[1 0.06749 0] Floors
        (CallFunction|MakeFloor (* _index_2 (Variables|Base|GetHeight)) (+ _index_2 1))))
    (:then_1
      ;;[1 0.03818 0] Checking if the building will have components
      (if (Variables|Checks|GetHasOutsidePillars?)
        ;;[0.02701 0 1] 4 Outside Pillars
        (for _index_3 (range 0 _returnvalue)
          (Components|InstancedStaticMesh|AddInstance _outerpillar (Math|Transform|MakeTransform (Math|Vector|MakeVector (* (Variables|Base|GetLength) 0.5) (* (Variables|Base|GetWidth) 0.5) (* _index_3 (Variables|Base|GetHeight))) "0, 0, 0" "1,1,1"))
          (Components|InstancedStaticMesh|AddInstance _outerpillar (Math|Transform|MakeTransform (Math|Vector|MakeVector (* (Variables|Base|GetLength) -0.5) (* (Variables|Base|GetWidth) -0.5) (* _index_3 (Variables|Base|GetHeight))) "0, 0, 0" "1,1,1"))
          (Components|InstancedStaticMesh|AddInstance _outerpillar (Math|Transform|MakeTransform (Math|Vector|MakeVector (* (Variables|Base|GetLength) -0.5) (* (Variables|Base|GetWidth) 0.5) (* _index_3 (Variables|Base|GetHeight))) "0, 0, 0" "1,1,1"))
          (Components|InstancedStaticMesh|AddInstance _outerpillar (Math|Transform|MakeTransform (Math|Vector|MakeVector (* (Variables|Base|GetLength) 0.5) (* (Variables|Base|GetWidth) -0.5) (* _index_3 (Variables|Base|GetHeight))) "0, 0, 0" "1,1,1")))))
    (:then_2
      (if (Variables|Checks|GetHasInsideHorizontalPillars?)
        ;;[1 1 1] Inside Pillars
        ;;;[0.1427 0.2344 0.1706] Horizontal Pillar
        (if (== (Math|Integer|%(Integer) _numberofhorizontalpillars 2) 0)
          _
          (else
            ;;;;[0.04278 1 0] Create Middle Pillar if Number of Pillar is odd number
            (CallFunction|MakePillar 0.0 0.0)))
        (for _index_4 (range 1 _returnvalue_2)
          (Components|InstancedStaticMesh|AddInstance _pillar_horizontal (Math|Transform|MakeTransform (Math|Vector|MakeVector (* _index_4 (Variables|Offsets|GetHorizontalPillarOffset)) 0.0 _returnvalue_5) "0, 0, 0" (Math|Vector|MakeVector 1.0 _returnvalue_4 1.0)))
          ;;;[1 0.1735 0] Vertical Pillar
          (if (Variables|Checks|GetHasInsideVerticalPillars?)
            (CallFunction|MakeVerticalPillar (* _index_4 (Variables|Offsets|GetHorizontalPillarOffset)))))
        (for _index_5 (range 1 _returnvalue_2)
          (bind _result (Math|Float|NegateFloat (* _index_5 (Variables|Offsets|GetHorizontalPillarOffset)))
            (:%20%20
              (Components|InstancedStaticMesh|AddInstance _pillar_horizontal (Math|Transform|MakeTransform (Math|Vector|MakeVector _result 0.0 _returnvalue_5) "0, 0, 0" (Math|Vector|MakeVector 1.0 _returnvalue_4 1.0)))
              (if (Variables|Checks|GetHasInsideVerticalPillars?)
                (CallFunction|MakeVerticalPillar _result)))))))
    (:then_3
      (if (Variables|Checks|GetHasRoof?)
        _))))

(fn MakeWall
  (params (LocationX :type Float%20%28single-precision%29) (LocationY :type Float%20%28single-precision%29) (RotationZ :type Float%20%28single-precision%29) (Height :type Float%20%28single-precision%29) (ScaleZ :type Float%20%28single-precision%29) (WallMeshInstance :type Instanced%20Static%20Mesh%20Component%20Object%20Reference))
  (bind _distortionangley (Variables|Offsets|GetdistortionAngleY))
  (bind _distortionanglex (Variables|Offsets|GetdistortionAngleX))
  (Components|InstancedStaticMesh|AddInstance WallMeshInstance (Math|Transform|MakeTransform (Math|Vector|MakeVector LocationX LocationY Height) (Math|Rotator|MakeRotator (Math|Random|RandomFloatinRange (* _distortionanglex -1.0) _distortionanglex) (Math|Random|RandomFloatinRange (* _distortionangley -1.0) _distortionangley) RotationZ) (Math|Vector|MakeVector 1.0 1.0 ScaleZ))))

(fn MakeFloor
  (params (Height :type Float%20%28single-precision%29) (Floor# :type Integer))
  (bind _returnvalue (* Floor# 4))
  (bind _returnvalue_2 (* Floor# 4))
  (bind _returnvalue_3 (* Floor# 4))
  (bind _returnvalue_4 (* Floor# 4))
  (bind _wallformingcurves (Variables|Curve|GetWallFormingCurves))
  (bind _wallformingcurves_2 (Variables|Curve|GetWallFormingCurves))
  (bind _wallformingcurves_3 (Variables|Curve|GetWallFormingCurves))
  (bind _wallformingcurves_4 (Variables|Curve|GetWallFormingCurves))
  (bind _returnvalue_5 (- _returnvalue_4 1))
  (bind _returnvalue_6 (- _returnvalue 4))
  (bind _returnvalue_7 (- _returnvalue_2 3))
  (bind _returnvalue_8 (- _returnvalue_3 2))
  (bind _output (Utilities|Array|Get(acopy) _wallformingcurves_3 _returnvalue_8))
  (bind _output_2 (Utilities|Array|Get(acopy) _wallformingcurves _returnvalue_5))
  (bind _output_3 (Utilities|Array|Get(acopy) _wallformingcurves_4 _returnvalue_6))
  (bind _output_4 (Utilities|Array|Get(acopy) _wallformingcurves_2 _returnvalue_7))
  (Utilities|FlowControl|Sequence
    (:then_0
      ;[1 1 1] Front Wall
      (for _index (range 0 (- (Math|Float|Truncate (/ (Variables|Base|GetWidth) (Variables|Base|GetDistanceBetweenWalls))) 1))
        ;;[0 0.3174 1] getting curve
        (Utilities|IsValid _output_3
          (:Is%20Valid
            (Variables|Curve|SetPreviousValidCurve_F _output_3))
          (:Is%20Not%20Valid
            _))
        (CallFunction|MakeWall (/ (Variables|Base|GetLength) 2.0) (- (+ (/ (Variables|Base|GetWidth) 2.0) (/ (Variables|Base|GetDistanceBetweenWalls) 2.0)) (* (+ _index 1) (Variables|Base|GetDistanceBetweenWalls))) (Variables|Default|GetrotationX) Height 1.0 (Utilities|Array|Get(acopy) (Variables|Mesh|GetMeshes_instances) (Math|Float|Truncate (+ (Math|Curves|GetFloatValue (Variables|Curve|GetPreviousValidCurve_F) (Math|Conversions|ToFloat(Integer) _index)) 0.1))))))
    (:then_1
      ;[1 1 1] Back Wall
      (for _index_2 (range 0 (- (Math|Float|Truncate (/ (Variables|Base|GetWidth) (Variables|Base|GetDistanceBetweenWalls))) 1))
        ;;[0 0.3174 1] getting curve
        (Utilities|IsValid _output_4
          (:Is%20Valid
            (Variables|Curve|SetPreviousValidCurve_B _output_4))
          (:Is%20Not%20Valid
            _))
        (CallFunction|MakeWall (/ (Variables|Base|GetLength) -2.0) (- (+ (/ (Variables|Base|GetWidth) 2.0) (/ (Variables|Base|GetDistanceBetweenWalls) 2.0)) (* (+ _index_2 1) (Variables|Base|GetDistanceBetweenWalls))) (* (Variables|Default|GetrotationX) -1.0) Height 1.0 (Utilities|Array|Get(acopy) (Variables|Mesh|GetMeshes_instances) (Math|Float|Truncate (+ (Math|Curves|GetFloatValue (Variables|Curve|GetPreviousValidCurve_B) (Math|Conversions|ToFloat(Integer) _index_2)) 0.1))))))
    (:then_2
      ;[1 1 1] Right Wall
      (for _index_3 (range 0 (- (Math|Float|Truncate (/ (Variables|Base|GetLength) (Variables|Base|GetDistanceBetweenWalls))) 1))
        ;;[0 0.3174 1] getting curve
        (Utilities|IsValid _output
          (:Is%20Valid
            (Variables|Curve|SetPreviousValidCurve_R _output))
          (:Is%20Not%20Valid
            _))
        (CallFunction|MakeWall (- (+ (/ (Variables|Base|GetLength) 2.0) (/ (Variables|Base|GetDistanceBetweenWalls) 2.0)) (* (+ _index_3 1) (Variables|Base|GetDistanceBetweenWalls))) (/ (Variables|Base|GetWidth) -2.0) (+ (Variables|Default|GetrotationY) 1.8e+02) Height 1.0 (Utilities|Array|Get(acopy) (Variables|Mesh|GetMeshes_instances) (Math|Float|Truncate (+ (Math|Curves|GetFloatValue (Variables|Curve|GetPreviousValidCurve_R) (Math|Conversions|ToFloat(Integer) _index_3)) 0.1))))))
    (:then_3
      ;[1 1 1] Left Wall
      (for _index_4 (range 0 (- (Math|Float|Truncate (/ (Variables|Base|GetLength) (Variables|Base|GetDistanceBetweenWalls))) 1))
        ;;[0 0.3174 1] getting curve
        (Utilities|IsValid _output_2
          (:Is%20Valid
            (Variables|Curve|SetPreviousValidCurve_L _output_2))
          (:Is%20Not%20Valid
            _))
        (CallFunction|MakeWall (- (+ (/ (Variables|Base|GetLength) 2.0) (/ (Variables|Base|GetDistanceBetweenWalls) 2.0)) (* (+ _index_4 1) (Variables|Base|GetDistanceBetweenWalls))) (/ (Variables|Base|GetWidth) 2.0) (Variables|Default|GetrotationY) Height 1.0 (Utilities|Array|Get(acopy) (Variables|Mesh|GetMeshes_instances) (Math|Float|Truncate (+ (Math|Curves|GetFloatValue (Variables|Curve|GetPreviousValidCurve_L) (Math|Conversions|ToFloat(Integer) _index_4)) 0.1))))))))

(fn MakeRoof
  (params (Height :type Float%20%28single-precision%29)))

(fn MakePillar
  (params (LocationX :type Float%20%28single-precision%29) (LocationY :type Float%20%28single-precision%29))
  ;[1 1 1] For Number of Pillars along axis
  (for _index (range 0 (- (Variables|Base|GetNumberOfHorizontalPillars) 1))
    ;[1 1 1] Create 1 pillar mesh per floor
    (for _index_2 (range 0 (- (Variables|Base|GetNumberOfFloors) 1))
      (Components|InstancedStaticMesh|AddInstance (Variables|Default|GetPillar_Vertical) (Math|Transform|MakeTransform (Math|Vector|MakeVector LocationX LocationY (* _index_2 (Variables|Base|GetHeight))) "0, 0, 0" (Math|Vector|MakeVector 1.0 1.0 1.0))))))

(fn MakeVerticalPillar
  (params (LocationX :type Float%20%28single-precision%29))
  (bind _numberofverticalpillars (Variables|Base|GetNumberOfVerticalPillars))
  (bind _returnvalue (/ _numberofverticalpillars 2))
  (if (== (Math|Integer|%(Integer) _numberofverticalpillars 2) 0)
    _
    (else
      ;[0.04278 1 0] Create Middle Pillar if Number of Pillar is odd number
      (CallFunction|MakePillar LocationX 0.0)))
  ;[1 0.653 0.5627] Positive Direction
  (for _index (range 1 _returnvalue)
    (CallFunction|MakePillar LocationX (* _index (Variables|Offsets|GetVerticalPillarOffset))))
  ;[1 0.653 0.5627] Negative Direction
  (for _index_2 (range 1 _returnvalue)
    (bind _result (Math|Float|NegateFloat (* _index_2 (Variables|Offsets|GetVerticalPillarOffset)))
      (:%20%20
        (CallFunction|MakePillar LocationX _result)))))