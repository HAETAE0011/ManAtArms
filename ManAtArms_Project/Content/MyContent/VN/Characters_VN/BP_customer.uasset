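; BP_customer is a customer that steers itself toward a Destination actor.
; Each Tick it uses kinematic arrive math, dividing the horizontal offset to the target by TimeToTarget to get a velocity while outside Radius.
; It sets location and facing directly, keeping its own height, but only when that velocity exceeds MaxSpeed and is clamped; slower velocities produce no movement.
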(event EventBeginPlay
  (|CallParentFunction))

(event EventTick
  (params (DeltaSeconds :type Float%20%28single-precision%29))
  (bind _destination (Variables|Default|GetDestination))
  (bind _destination_2 (Variables|Default|GetDestination))
  (bind _returnvalue (Transformation|GetActorLocation _destination))
  (bind _returnvalue_2 (Transformation|GetActorLocation _destination_2))
  (|CallParentFunction DeltaSeconds)
  (Utilities|IsValid _destination_2
    (:Is%20Valid
      (if (> (Math|Vector|VectorLength (- (Math|Vector|MakeVector (.x _returnvalue_2) (.y _returnvalue_2) (.z (Transformation|GetActorLocation))) (Transformation|GetActorLocation))) (Variables|Default|GetRadius))
        (bind _output_get (Variables|Default|Setvelocity (/ (- (Math|Vector|MakeVector (.x _returnvalue) (.y _returnvalue) (.z (Transformation|GetActorLocation))) (Transformation|GetActorLocation)) (Variables|Default|GetTimeToTarget))))
        (if (> (Math|Vector|VectorLength _output_get) (Variables|Default|GetMaxSpeed))
          (Variables|Default|Setvelocity (* (Math|Vector|Normalize (Variables|Default|Getvelocity)) (Variables|Default|GetMaxSpeed)))
          (Transformation|SetActorLocationAndRotation (+ (Transformation|GetActorLocation) (* (Variables|Default|Getvelocity) DeltaSeconds)) (Math|Rotator|MakeRotfromX (Variables|Default|Getvelocity))))))))

(fn ConstructionScript
  (|CallParentFunction))