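; BP_Noodle is a noodle dish prop built from separate noodle, sauce and topping static mesh components.
; SetNoodleMeshes maps the NoodleType variable to one of six preset combinations of mesh array indices.
; SetMeshes applies those indices in a chain of validity checks, so an invalid mesh also skips the components after it.
; The construction script is empty, and the file shows no caller for SetNoodleMeshes.
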(fn ConstructionScript)

(fn SetNoodleMeshes
  (switch int (Variables|Default|GetNoodleType)
    (:1
      (CallFunction|SetMeshes))
    (:2
      (CallFunction|SetMeshes 0 1 1))
    (:3
      (CallFunction|SetMeshes 1 2 3))
    (:4
      (CallFunction|SetMeshes 1 1 3))
    (:5
      (CallFunction|SetMeshes 2 1 2))
    (:6
      (CallFunction|SetMeshes 2 1 4))))

(fn SetMeshes
  (params (NoodleType :type Integer) (SauceType :type Integer) (ToppingType :type Integer))
  (bind _noodle_meshes (Variables|Default|GetNoodle_Meshes))
  (bind _sauce_meshes (Variables|Default|GetSauce_Meshes))
  (bind _topping_meshes (Variables|Default|GetTopping_Meshes))
  (bind _output (Utilities|Array|Get(acopy) _topping_meshes ToppingType))
  (bind _output_2 (Utilities|Array|Get(acopy) _noodle_meshes NoodleType))
  (bind _output_3 (Utilities|Array|Get(acopy) _sauce_meshes SauceType))
  (Utilities|IsValid _output_2
    (:Is%20Valid
      (Components|StaticMesh|SetStaticMesh (Variables|Default|GetNoodle) _output_2)
      (Utilities|IsValid _output_3
        (:Is%20Valid
          (Components|StaticMesh|SetStaticMesh (Variables|Default|GetSauce) _output_3)
          (Utilities|IsValid _output
            (:Is%20Valid
              (Components|StaticMesh|SetStaticMesh (Variables|Default|GetTopping) _output))))))))