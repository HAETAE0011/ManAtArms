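; Procedural pipe generator that builds spline meshes along an editable spline in the Construction Script.
; Regulate resamples the middle of the spline at a set segment length into a temporary spline, keeping end points, then destroys it after meshing.
; Otherwise each spline segment gets a scaled mesh, with optional evenly spaced instanced submeshes.
; SplineMeshCreation offers start/middle/end meshing but is not called here.
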(event EventBeginPlay)

(event Collision|EventActorBeginOverlap
  (params (OtherActor :type Actor%20Object%20Reference)))

(event EventTick
  (params (DeltaSeconds :type Float%20%28single-precision%29)))

(fn ConstructionScript
  (bind _spline (Variables|Default|GetSpline))
  (bind _lengthpereachspline (Variables|Default|GetLengthPerEachSpline))
  (bind _spline_2 (Variables|Default|GetSpline))
  (bind _scale (Variables|Base|GetScale))
  (bind _scale_2 (Variables|Base|GetScale))
  (bind _numberofsubmeshes (Variables|Base|GetNumberOfSubmeshes))
  (bind _returnvalue (Math|Vector2D|MakeVector2D _scale _scale))
  (bind _returnvalue_2 (Spline|GetNumberOfSplinePoints _spline))
  (bind _returnvalue_3 (Spline|GetDistanceAlongSplineatSplinePoint _spline 1))
  (bind _returnvalue_4 (- _returnvalue_2 1))
  (bind _returnvalue_5 (- _returnvalue_4 2))
  (bind _returnvalue_6 (Spline|GetDistanceAlongSplineatSplinePoint _spline _returnvalue_5))
  (Components|StaticMesh|SetStaticMesh (Variables|Default|GetSubMesh) (Variables|Meshes|GetMeshesOnSpline))
  ;[1 1 1] Refresh function
  (if (Variables|Base|GetRefresh)
    (Variables|Base|SetRefresh false)
    (Class|KismetMathLibrary|SeedRandomStream (Variables|Default|GetRandomSeed)))
  (if (Variables|Base|GetRegulate?)
    ;[1 1 1] Only one Spline
    (bind _returnvalue_7 (AddComponent|AddSplineComponent false))
    (Spline|ClearSplinePoints _returnvalue_7 true)
    (Variables|Default|SetDistanceBetweenSubmeshsChecker 0.0)
    (for _index (range 0 _returnvalue_4)
      ;;[1 1 1] Initial 2 point
      (if (<= _index 1)
        (Spline|AddSplinePoint _returnvalue_7 (Spline|GetLocationatSplinePoint _spline _index "World") "World" true)))
    ;;[1 1 1] Regulate the distance between points in spline
    (for _index_2 (range 0 (Math|Float|Truncate (- _returnvalue_6 _returnvalue_3)))
      (if (or (<= _returnvalue_6 (Variables|Default|GetDistanceBetweenSubmeshsChecker)) (>= _returnvalue_3 (Variables|Default|GetDistanceBetweenSubmeshsChecker)))
        _
        (else
          (Spline|AddSplinePoint _returnvalue_7 (Spline|GetLocationatDistanceAlongSpline _spline (* _index_2 _lengthpereachspline) "World") "World" true)))
      (Variables|Default|SetDistanceBetweenSubmeshsChecker (+ (Variables|Default|GetDistanceBetweenSubmeshsChecker) _lengthpereachspline)))
    ;;[1 1 1] Last 2 point
    (for _index_3 (range 0 _returnvalue_4)
      (if (>= _index_3 (- _returnvalue_4 2))
        (Spline|AddSplinePoint _returnvalue_7 (Spline|GetLocationatSplinePoint _spline _index_3 "World") "World" true)))
    ;;[0.3098 0.2078 1] Create Spline Mesh
    (for _index_4 (range 0 (- (Spline|GetNumberOfSplinePoints _returnvalue_7) 2))
      (bind _returnvalue_8 (AddComponent|AddSplineMeshComponent false))
      (Components|StaticMesh|SetStaticMesh _returnvalue_8 (Variables|Meshes|GetSplineMesh))
      (SplineMesh|SetStartandEnd _returnvalue_8 (Spline|GetLocationatSplinePoint _returnvalue_7 _index_4 "Local") (Spline|GetTangentatSplinePoint _returnvalue_7 _index_4 "Local") (Spline|GetLocationatSplinePoint _returnvalue_7 (+ _index_4 1) "Local") (Spline|GetTangentatSplinePoint _returnvalue_7 (+ _index_4 1) "Local") true :!class /Script/Engine.SplineMeshComponent))
    ;;[0.25 0.03448 0.2014] At the end, Clear the splines/points created
    (Spline|ClearSplinePoints _returnvalue_7 true)
    (Components|DestroyComponent _returnvalue_7)
    (else
      ;[0.3098 0.2078 1] Create Spline Mesh
      (for _index_5 (range 0 (- (Spline|GetNumberOfSplinePoints _spline_2) 2))
        (bind _returnvalue_9 (AddComponent|AddSplineMeshComponent false))
        (SplineMesh|SetStartScale _returnvalue_9 _returnvalue true :!class /Script/Engine.SplineMeshComponent)
        (SplineMesh|SetEndScale _returnvalue_9 _returnvalue true :!class /Script/Engine.SplineMeshComponent)
        (Components|StaticMesh|SetStaticMesh _returnvalue_9 (Variables|Meshes|GetSplineMesh))
        (SplineMesh|SetStartandEnd _returnvalue_9 (Spline|GetLocationatSplinePoint _spline_2 _index_5 "Local") (Spline|GetTangentatSplinePoint _spline_2 _index_5 "Local") (Spline|GetLocationatSplinePoint _spline_2 (+ _index_5 1) "Local") (Spline|GetTangentatSplinePoint _spline_2 (+ _index_5 1) "Local") true :!class /Script/Engine.SplineMeshComponent))
      (if (and (Variables|Base|GetShowSubMesh) (> _numberofsubmeshes 0))
        (for _index_6 (range 0 (- _numberofsubmeshes 1))
          (Class|InstancedStaticMeshComponent|AddInstanceWorldSpace (Variables|Default|GetSubMesh) (Math|Transform|MakeTransform (Spline|GetLocationatDistanceAlongSpline _spline_2 (* _index_6 (/ (Spline|GetSplineLength _spline_2) (Math|Conversions|ToFloat(Integer) (Variables|Base|GetNumberOfSubmeshes)))) "World") (Spline|GetRotationatDistanceAlongSpline _spline_2 (* _index_6 (/ (Spline|GetSplineLength _spline_2) (Math|Conversions|ToFloat(Integer) (Variables|Base|GetNumberOfSubmeshes)))) "World") (Math|Vector|MakeVector _scale_2 _scale_2 _scale_2))))))))

(fn SplineMeshCreation
  (params (Spline :type Spline%20Component%20Object%20Reference) (Start :type Static%20Mesh%20Object%20Reference) (Middle :type Static%20Mesh%20Object%20Reference) (End :type Static%20Mesh%20Object%20Reference))
  (bind _returnvalue (Spline|GetNumberOfSplinePoints Spline))
  (bind _returnvalue_2 (- _returnvalue 2))
  ;[1 1 1] Spline Mesh
  (for _index (range 0 _returnvalue_2)
    (bind _returnvalue_3 (AddComponent|AddSplineMeshComponent false))
    (if (== _index 0)
      ;;[1 0.4688 0.4688] Three Meshes- start, middle, end
      (Components|StaticMesh|SetStaticMesh _returnvalue_3 Start)
      (elif (== _returnvalue_2 _index)
        (Components|StaticMesh|SetStaticMesh _returnvalue_3 End)
        (else
          (Components|StaticMesh|SetStaticMesh _returnvalue_3 Middle))))
    (SplineMesh|SetStartandEnd _returnvalue_3 (Spline|GetLocationatSplinePoint Spline _index "Local") (Spline|GetTangentatSplinePoint Spline _index "Local") (Spline|GetLocationatSplinePoint Spline (+ _index 1) "Local") (Spline|GetTangentatSplinePoint Spline (+ _index 1) "Local") true :!class /Script/Engine.SplineMeshComponent)))