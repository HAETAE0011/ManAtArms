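; Construction-script actor that scatters a chosen static mesh along a spline as instanced static mesh instances.
; It divides the spline length into equal segments, one per mesh, and randomizes each instance's position within its segment.
; Each instance combines a base rotation with random per-axis offsets, at unit scale.
; Every construction run reseeds the stream and reshuffles the layout, with Refresh serving as a self-resetting rerun toggle.
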(event EventBeginPlay)

(event Collision|EventActorBeginOverlap
  (params (OtherActor :type Actor%20Object%20Reference)))

(event EventTick
  (params (DeltaSeconds :type Float%20%28single-precision%29)))

(fn ConstructionScript
  (bind _spline (Variables|Default|GetSpline))
  (bind _randomlocationoffset (Variables|Default|GetRandomLocationOffset))
  (bind _numberofmeshes (Variables|Default|GetNumberOfMeshes))
  (bind _randomrotoffset (Variables|Default|GetRandomRotOffset))
  (bind (_x _y _z) (Math|Vector|BreakVector _randomrotoffset))
  (bind _returnvalue (Spline|GetSplineLength _spline))
  (Components|StaticMesh|SetStaticMesh (Variables|Default|GetInstancedStaticMesh) (Variables|Default|GetMeshesOnSpline))
  (Components|InstancedStaticMesh|ClearInstances (Variables|Default|GetInstancedStaticMesh))
  ;[1 1 1] Refresh function
  (if (Variables|Default|GetRefresh)
    (Variables|Default|SetRefresh false))
  (Class|KismetMathLibrary|SeedRandomStream (Variables|Default|GetRandomSeed))
  (if (> (Variables|Default|GetNumberOfMeshes) 0)
    (for _index (range 0 (- (Variables|Default|GetNumberOfMeshes) 1))
      (Components|InstancedStaticMesh|AddInstance (Variables|Default|GetInstancedStaticMesh) (Math|Transform|MakeTransform (Spline|GetLocationatDistanceAlongSpline _spline (+ (* _index (/ _returnvalue (Math|Conversions|ToFloat(Integer) _numberofmeshes))) (* (Math|Random|RandomIntegerinRangefromStream (+ _randomlocationoffset 0) (- 100 _randomlocationoffset) (Variables|Default|GetRandomSeed)) (/ _returnvalue (Math|Conversions|ToFloat(Integer) (* _numberofmeshes 100))))) "Local") (Math|Rotator|CombineRotators (Variables|Default|GetRotation) (Math|Rotator|MakeRotator (Math|Random|RandomFloatinRange (* _x -1.0) _x) (Math|Random|RandomFloatinRange (* _y -1.0) _y) (Math|Random|RandomFloatinRange (* _z -1.0) _z))))))))