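; Procedural building actor that builds stacked floor groups along a spline footprint in the construction script.
; Each spline segment is subdivided by facade mesh length through a temporary spline, placing spline-mesh walls per storey and instanced pillars at segment starts.
; Optional ceiling and bottom cap are procedural-mesh triangle fans from the local origin, with the ceiling at a separate Height value.
; SplineMeshCreation, a start/middle/end mesh helper, is not called here.
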(event EventBeginPlay)

(event Collision|EventActorBeginOverlap
  (params (OtherActor :type Actor%20Object%20Reference)))

(event EventTick
  (params (DeltaSeconds :type Float%20%28single-precision%29)))

(fn ConstructionScript
  (bind _floors (Variables|Default|GetFloors))
  (bind _bottomcap (Variables|Default|GetBottomCap))
  (bind _spline (Variables|Default|GetSpline))
  (bind _spline_2 (Variables|Default|GetSpline))
  (bind _ceiling (Variables|Default|GetCeiling))
  (bind _spline_3 (Variables|Default|GetSpline))
  (bind _spline_4 (Variables|Default|GetSpline))
  (bind _returnvalue (Utilities|Array|Length _floors))
  ;[1 1 1] Refresh function
  (if (Variables|Base|GetRefresh)
    (Variables|Base|SetRefresh false))
  (Utilities|FlowControl|Sequence
    (:then_0
      (if (> _returnvalue 0)
        (Variables|Default|SetTMP_height 0.0)
        (for _index (range 0 (- (Spline|GetNumberOfSplinePoints _spline_3) 1))
          (Spline|SetSplinePointType _spline_3 _index (Variables|Base|GetSplinePointType) true))
        ;[1 1 1] Floors
        (for _index_2 (range 0 (- _returnvalue 1))
          (if (> (Spline|GetNumberOfSplinePoints _spline) 0)
            ;[1 1 1] For each point of spline
            (for _index_3 (range 0 (- (Spline|GetNumberOfSplinePoints _spline) 1))
              (bind _returnvalue_2 (AddComponent|AddSplineComponent false))
              (Spline|ClearSplinePoints _returnvalue_2 true)
              (for _index_4 (range 0 (Math|Float|Round (/ (- (Spline|GetDistanceAlongSplineatSplinePoint _spline (+ _index_3 1)) (Spline|GetDistanceAlongSplineatSplinePoint _spline _index_3)) (.Facade_Mesh_Length (Utilities|Struct|BreakST_Floor (Utilities|Array|Get(acopy) _floors _index_2))))))
                (Spline|AddSplinePoint _returnvalue_2 (Spline|GetLocationatDistanceAlongSpline _spline (+ (Spline|GetDistanceAlongSplineatSplinePoint _spline _index_3) (* _index_4 (/ (- (Spline|GetDistanceAlongSplineatSplinePoint _spline (+ _index_3 1)) (Spline|GetDistanceAlongSplineatSplinePoint _spline _index_3)) (Math|Conversions|ToFloat(Integer) (Math|Float|Round (/ (- (Spline|GetDistanceAlongSplineatSplinePoint _spline (+ _index_3 1)) (Spline|GetDistanceAlongSplineatSplinePoint _spline _index_3)) (.Facade_Mesh_Length (Utilities|Struct|BreakST_Floor (Utilities|Array|Get(acopy) _floors _index_2))))))))) "World") "World" true))
              (Utilities|IsValid (Utilities|Array|Get(acopy) (Variables|Meshes|GetPillarMeshList) (.Pillar_Type (Utilities|Struct|BreakST_Floor (Utilities|Array|Get(acopy) _floors _index_2))))
                (:Is%20Valid
                  (bind _returnvalue_3 (AddComponent|AddInstancedStaticMeshComponent false))
                  (Components|StaticMesh|SetStaticMesh _returnvalue_3 (Utilities|Array|Get(acopy) (Variables|Meshes|GetPillarMeshList) (.Pillar_Type (Utilities|Struct|BreakST_Floor (Utilities|Array|Get(acopy) _floors _index_2)))))
                  (for _index_5 (range 0 (- (.NumberOfFloors (Utilities|Struct|BreakST_Floor (Utilities|Array|Get(acopy) _floors _index_2))) 1))
                    (Components|InstancedStaticMesh|AddInstance _returnvalue_3 (Math|Transform|MakeTransform (+ (Spline|GetLocationatSplinePoint _returnvalue_2 0 "Local") (Math|Vector|MakeVector 0.0 0.0 (+ (* (.floorHeight (Utilities|Struct|BreakST_Floor (Utilities|Array|Get(acopy) _floors _index_2))) (Math|Conversions|ToFloat(Integer) _index_5)) (Variables|Default|GetTMP_height) -0.05)))))))
                (:Is%20Not%20Valid
                  _))
              ;[1 1 1] Wall
              (for _index_6 (range 0 (- (.NumberOfFloors (Utilities|Struct|BreakST_Floor (Utilities|Array|Get(acopy) _floors _index_2))) 1))
                (for _index_7 (range 0 (- (Spline|GetNumberOfSplinePoints _returnvalue_2) 1))
                  (Spline|SetSplinePointType _returnvalue_2 _index_7 (Variables|Base|GetSplinePointType) true)
                  (bind _returnvalue_4 (AddComponent|AddSplineMeshComponent false))
                  (SplineMesh|SetForwardAxis _returnvalue_4 (Variables|Default|GetForwardAxis) true)
                  (Components|StaticMesh|SetStaticMesh _returnvalue_4 (Utilities|Array|Get(acopy) (Variables|Meshes|GetWallMeshList) (.facade_Type (Utilities|Struct|BreakST_Floor (Utilities|Array|Get(acopy) _floors _index_2)))))
                  (SplineMesh|SetStartandEnd _returnvalue_4 (+ (Spline|GetLocationatSplinePoint _returnvalue_2 _index_7 "Local") (Math|Vector|MakeVector 0.0 0.0 (+ (* (.floorHeight (Utilities|Struct|BreakST_Floor (Utilities|Array|Get(acopy) _floors _index_2))) (Math|Conversions|ToFloat(Integer) _index_6)) (Variables|Default|GetTMP_height)))) (Spline|GetTangentatSplinePoint _returnvalue_2 _index_7 "Local") (+ (Spline|GetLocationatSplinePoint _returnvalue_2 (+ _index_7 1) "Local") (Math|Vector|MakeVector 0.0 0.0 (+ (* (.floorHeight (Utilities|Struct|BreakST_Floor (Utilities|Array|Get(acopy) _floors _index_2))) (Math|Conversions|ToFloat(Integer) _index_6)) (Variables|Default|GetTMP_height)))) (Spline|GetTangentatSplinePoint _returnvalue_2 _index_7 "Local") true :!class /Script/Engine.SplineMeshComponent)))
              (Spline|ClearSplinePoints _returnvalue_2 true)
              (Components|DestroyComponent _returnvalue_2))
            (Variables|Default|SetTMP_height (+ (Variables|Default|GetTMP_height) (* (.NumberOfFloors (Utilities|Struct|BreakST_Floor (Utilities|Array|Get(acopy) _floors _index_2))) (.floorHeight (Utilities|Struct|BreakST_Floor (Utilities|Array|Get(acopy) _floors _index_2))))))))))
    (:then_1
      ;[1 1 1] Procedurally generated ceiling
      (if (Variables|Base|GetHasCeiling)
        (for _index_8 (range 0 (- (Spline|GetNumberOfSplinePoints _spline_2) 1))
          (Class|ProceduralMeshComponent|CreateMeshSectionLinearColor _ceiling _index_8 (Utilities|Array|MakeArray (Math|Vector|MakeVector 0.0 0.0 (Variables|Default|Getheight)) (+ (Spline|GetLocationatSplinePoint _spline_2 _index_8 "Local") (Math|Vector|MakeVector 0.0 0.0 (Variables|Default|Getheight))) (+ (Spline|GetLocationatSplinePoint _spline_2 (+ _index_8 1) "Local") (Math|Vector|MakeVector 0.0 0.0 (Variables|Default|Getheight)))) (Utilities|Array|MakeArray 0 1 2) 0 (Utilities|Array|MakeArray "" "(X=0.000000,Y=1.000000)" "(X=1.000000,Y=0.000000)" "(X=1.000000,Y=1.000000)") 0 0 0 0 0 true)
          (Rendering|Material|SetMaterial _ceiling _index_8 (Variables|Default|GetCeilingMaterial)))))
    (:then_2
      ;[1 1 1] Procedurally generated ground cap
      (if (Variables|Base|GetHasBottomCap)
        (for _index_9 (range 0 (- (Spline|GetNumberOfSplinePoints _spline_4) 1))
          (Class|ProceduralMeshComponent|CreateMeshSectionLinearColor _bottomcap _index_9 (Utilities|Array|MakeArray (Math|Vector|MakeVector 0.0 0.0 0.0) (Spline|GetLocationatSplinePoint _spline_4 _index_9 "Local") (Spline|GetLocationatSplinePoint _spline_4 (+ _index_9 1) "Local")) (Utilities|Array|MakeArray 0 1 2) 0 (Utilities|Array|MakeArray "" "(X=0.000000,Y=1.000000)" "(X=1.000000,Y=0.000000)" "(X=1.000000,Y=1.000000)") 0 0 0 0 0 true)
          (Rendering|Material|SetMaterial _bottomcap _index_9 (Variables|Default|GetCeilingMaterial)))))))

(fn SplineMeshCreation
  (params (Spline :type Spline%20Component%20Object%20Reference) (Start :type Static%20Mesh%20Object%20Reference) (Middle :type Static%20Mesh%20Object%20Reference) (End :type Static%20Mesh%20Object%20Reference))
  (bind _returnvalue (Spline|GetNumberOfSplinePoints Spline))
  (bind _returnvalue_2 (- _returnvalue 2))
  ;[1 1 1] Spline Mesh
  (for _index (range 0 _returnvalue_2)
    (bind _returnvalue_3 (AddComponent|AddSplineMeshComponent false))
    (if (== _index 0)
      ;;[1 0.4688 0.4688] Three Meshes- start, middle, end
      (Components|StaticMesh|SetStaticMesh _returnvalue_3 Start)
      (elif (== _returnvalue_2 _index)
        (Components|StaticMesh|SetStaticMesh _returnvalue_3 End)
        (else
          (Components|StaticMesh|SetStaticMesh _returnvalue_3 Middle))))
    (SplineMesh|SetStartandEnd _returnvalue_3 (Spline|GetLocationatSplinePoint Spline _index "Local") (Spline|GetTangentatSplinePoint Spline _index "Local") (Spline|GetLocationatSplinePoint Spline (+ _index 1) "Local") (Spline|GetTangentatSplinePoint Spline (+ _index 1) "Local") true :!class /Script/Engine.SplineMeshComponent)))