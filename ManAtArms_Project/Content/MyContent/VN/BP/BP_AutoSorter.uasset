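; BP_AutoSorter is a construction-script actor that procedurally stacks random static meshes along a chosen axis.
; It creates an instanced mesh component per supplied mesh, then adds stream-randomized instances with position and angle distortion, yaw and XY scale variation.
; Each step advances by the chosen mesh's height divided by the cosine of the X tilt.
; The Refresh toggle reseeds the stream and resets the accumulated height.
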(event EventBeginPlay)

(event Collision|EventActorBeginOverlap
  (params (OtherActor :type Actor%20Object%20Reference)))

(event EventTick
  (params (DeltaSeconds :type Float%20%28single-precision%29)))

(fn ConstructionScript
  (bind _randomseed (Variables|Default|GetRandomSeed))
  (bind _distortionanglex (Variables|RandomVariables|GetDistortionAngleX))
  (bind _meshes (Variables|FixedVariables|GetMeshes))
  (bind _meshes_instances (Variables|Default|GetMeshes_instances))
  (bind _distortionangley (Variables|RandomVariables|GetDistortionAngleY))
  (bind _meshes_instances_2 (Variables|Default|GetMeshes_instances))
  (bind _rotationx (Variables|FixedVariables|GetrotationX))
  ;[1 1 1] Setting Instanced static mesh component array to given static mesh array
  (Utilities|Array|Clear _meshes_instances)
  (for _index (range 0 (Utilities|Array|LastIndex _meshes))
    (bind _returnvalue (AddComponent|AddInstancedStaticMeshComponent false))
    (Components|StaticMesh|SetStaticMesh _returnvalue (Utilities|Array|Get(acopy) _meshes _index))
    (Utilities|Array|Add _meshes_instances _returnvalue))
  (switch Utilities|FlowControl|Switch|SwitchonAxisTypes (Variables|FixedVariables|GetForward%20Axis)
    (:NewEnumerator0
      (Variables|FixedVariables|SetForwardAxis "1.000000, 0, 0"))
    (:NewEnumerator1
      (Variables|FixedVariables|SetForwardAxis "0,1.000000, 0"))
    (:NewEnumerator3
      (Variables|FixedVariables|SetForwardAxis "0, 0,1.000000")))
  (if (Variables|Base|Getrefresh)
    (Variables|Base|Setrefresh false)
    (Class|KismetMathLibrary|SeedRandomStream (Variables|Default|GetRandomSeed))
    (Variables|Default|SettotalHeight 0.0)
    (else
      (Utilities|FlowControl|DoOnce false
        (:Completed
          _))))
  (for _index_2 (range 1 (Variables|Base|GetnumberOfInstances))
    (bind _output_get (LocalVariables|SetRandomInt (Math|Random|RandomIntegerinRangefromStream 0 (Utilities|Array|LastIndex _meshes_instances_2) _randomseed)))
    (bind _output_get_2 (Variables|Default|SetRandomRotationValue (Math|Random|RandomFloatinRangefromStream (Variables|RandomVariables|GetMinimumRotationZ) (Variables|RandomVariables|GetMaximumRotationZ) _randomseed)))
    (bind _output_get_3 (Variables|Default|SetRandomscaleValueX (Math|Random|RandomFloatinRangefromStream (Variables|RandomVariables|GetMinimumSize_X) (Variables|RandomVariables|GetMaximumSize_X) _randomseed)))
    (bind _output_get_4 (Variables|Default|SetRandomscaleValueY (Math|Random|RandomFloatinRangefromStream (Variables|RandomVariables|GetMinimumSize_Y) (Variables|RandomVariables|GetMaximumSize_Y) _randomseed)))
    (Components|InstancedStaticMesh|AddInstance (Utilities|Array|Get(acopy) _meshes_instances_2 _output_get) (Math|Transform|MakeTransform (+ (Math|Vector|MakeVector (Math|Random|RandomFloatinRangefromStream (* -1 (Variables|RandomVariables|GetDistortionOffsetX)) (Variables|RandomVariables|GetDistortionOffsetX) _randomseed) (Math|Random|RandomFloatinRangefromStream (* -1 (Variables|RandomVariables|GetDistortionOffsetY)) (Variables|RandomVariables|GetDistortionOffsetY) _randomseed) 0.0) (* (Variables|FixedVariables|GetForwardAxis) (Variables|Default|GettotalHeight))) (Math|Rotator|MakeRotator (+ _rotationx (Math|Random|RandomFloatinRangefromStream (* _distortionanglex -1.0) _distortionanglex _randomseed)) (Math|Random|RandomFloatinRangefromStream (* _distortionangley -1.0) _distortionangley _randomseed) _output_get_2) (Math|Vector|MakeVector _output_get_3 _output_get_4 1.0)))
    (Variables|Default|SettotalHeight (+ (Variables|Default|GettotalHeight) (/ (Utilities|Array|Get(acopy) (Variables|FixedVariables|GetMeshHeights) _output_get) (Math|Trig|Cos(Degrees) _rotationx))))))