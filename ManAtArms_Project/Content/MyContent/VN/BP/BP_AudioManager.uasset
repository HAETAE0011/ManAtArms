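; BP_AudioManager is an audio manager Blueprint in the VN folder that handles background music and holds a rain sound.
; On BeginPlay it creates 2D audio components for both sounds and stores them in variables.
; The PlayBGM? event plays the music from the start or stops it, based on its Play flag.
; The rain component is never started here, as its Play call is unconnected.
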(event Custom|PlayBGM?
  (params (Play? :type Boolean))
  (bind _sound2d_bgm (Variables|Default|GetSound2D_BGM))
  (if Play?
    (Audio|Components|Audio|Play _sound2d_bgm 0.0)
    (else
      (Audio|Components|Audio|Stop _sound2d_bgm))))

(event EventBeginPlay
  (bind _returnvalue (Audio|CreateSound2D (Variables|Default|GetrainSound) 1.0 1.0 0.0 0 false false))
  (bind _output_get (Variables|Default|SetSound2D_Rain _returnvalue))
  (bind _returnvalue_2 (Audio|CreateSound2D (Variables|Default|GetBackgroundMusic) 1.0 1.0 0.0 0 false false))
  (Variables|Default|SetSound2D_BGM _returnvalue_2))

(fn ConstructionScript)