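; Game manager for a visual novel with a food-and-drink serving game, switching between menu, story, customer, gameplay and result turns.
; Turn events create the story or gameplay widgets, spawn random orders, cycle cameras and fire dispatchers for UI updates.
; During gameplay, Tick drains the latest customer's satisfaction and handles cooldowns, while helpers check orders and daily customer limits.
; The construction script loads story scripts from DataTables; the ending branch is empty.
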(event Custom|ChangeCameraTo
  (params (CameraNum :type Integer))
  ;[0 0.3098 1] Camera
  (if (< CameraNum (Variables|Default|GetMaxCamNum))
    (Variables|Default|SetCameraNum CameraNum)
    (Default|CallChangeCameraEventDispatcher)))

(event Custom|UI_Cam
  ;[0 0.3098 1] Camera
  (CallFunction|ChangeCamera)
  (Default|CallChangeCameraEventDispatcher))

(event Custom|StartStoryTurn
  ;[0.5781 0.5781 0.5781] Manage Turns
  ;;[1 1 1] Story Mode
  (Variables|Default|SetlastCustomerIndexToday 0)
  (Variables|Default|SetTurn_Type "NewEnumerator1")
  (Utilities|Platform|CollectGarbage)
  (bind _returnvalue (UserInterface|CreateWidget "/Game/MyContent/VN/UI/UI_VN_Story.UI_VN_Story_C" (Game|GetPlayerController 0)))
  (Variables|/Game/MyContent/VN/UI/UI_VN_Story.UI_VN_Story_C|SetPlayer _returnvalue self)
  (UserInterface|Viewport|AddtoViewport _returnvalue 0)
  (Default|CallUIAnimationEventDispatcher)
  ;;;[1 0 0] if day reaches to the date_end, show the ending
  (if (>= (Variables|Default|GetCurrentDay) 3)
    _))

(event Custom|ChangeCamera
  ;[0 0.3098 1] Camera
  (if (< (Variables|Default|GetCameraNum) (Variables|Default|GetMaxCamNum))
    (Variables|Default|SetCameraNum (+ (Variables|Default|GetCameraNum) 1))
    (else
      (Variables|Default|SetCameraNum 1))))

(event Custom|CustomerTurnStart
  ;[0.5781 0.5781 0.5781] Manage Turns
  ;;[0 0.2626 1] GamePlay
  ;;;[1 0 0] CustomerTurn
  (Class|VNPlayerParent|AddCustomer "" (Math|Random|RandomIntegerinRange 1 6) (Math|Random|RandomIntegerinRange 1 5))
  (Variables|Default|SetTurn_type "NewEnumerator5")
  (Default|CallUIAnimationEventDispatcher))

(event Custom|StartGameTurn
  ;[0.5781 0.5781 0.5781] Manage Turns
  ;;[0 0.2626 1] GamePlay
  ;;;[0.5713 0 1] Set Today's max customers
  (bind _result (Math|Integer|IncrementInt (Variables|Default|GetCurrentDay))
    (:%20%20
      (Variables|Default|SetMaxCustomerNum (Utilities|Array|Get(acopy) (Variables|Default|GetDayMaxCustomers) (- _result 1)))
      (bind _returnvalue (UserInterface|CreateWidget "/Game/MyContent/VN/UI/UI_VN_GamePlay_refined.UI_VN_GamePlay_refined_C" (Game|GetPlayerController 0)))
      (Variables|/Game/MyContent/VN/UI/UI_VN_GamePlay_refined.UI_VN_GamePlay_refined_C|SetPlayer _returnvalue self)
      (UserInterface|Viewport|AddtoViewport _returnvalue 0)
      (CallFunction|ChangeCamerato 1)
      (CallFunction|CustomerTurnStart))))

(event EventBeginPlay
  ;[1 0 0] BeginPlay
  ;;[1 1 1] Initialize
  (Variables|Default|SetTurn_Type "NewEnumerator3")
  (Variables|Default|Setmoney (Variables|Default|GetinitialMoney)))

(event EventTick
  (params (DeltaSeconds :type Float%20%28single-precision%29))
  ;[0.4366 0.4713 1] OnTickEvent
  (switch Utilities|FlowControl|Switch|SwitchonTurnType (Variables|Default|GetTurn_Type)
    (:NewEnumerator0
      (CallFunction|CalculateSatisfactionLevel DeltaSeconds)
      (Class|VNPlayerParent|HandleCooldown DeltaSeconds))))

(fn ConstructionScript
  (Utilities|Array|Clear (Variables|Default|Getstory_day1_opening))
  (Utilities|Array|Clear (Variables|Default|Getstory_day1))
  (Utilities|Array|Clear (Variables|Default|Getstory_day2))
  (Utilities|Array|Clear (Variables|Default|Getstory_day3))
  (CallFunction|GetScript (Variables|Default|GetDay1_openingScript) (Variables|Default|GetDay1_Script) (Variables|Default|GetDay2_Script) (Variables|Default|GetDay3_Script)))

(fn CalculateSatisfactionLevel
  (params (deltaTime :type Float%20%28single-precision%29))
  (bind _customers (Variables|Default|Getcustomers))
  (bind _returnvalue (Utilities|Array|LastIndex _customers))
  (bind _output (Utilities|Array|Get(acopy) _customers _returnvalue))
  (bind _satisfactionlevel (Utilities|Struct|BreakCustomer_struct _output))
  (if (>= _satisfactionlevel 0.0)
    (Utilities|Struct|SetmembersinCustomer_struct _output (- _satisfactionlevel (* deltaTime (Variables|Default|GetsatisfactionMultiplier))))
    (else
      (Utilities|Struct|SetmembersinCustomer_struct _output 0.0))))

(fn CheckPlayTurnEnd
  (bind _lastcustomerindextoday (Variables|Default|GetlastCustomerIndexToday))
  (bind _daymaxcustomers (Variables|Default|GetDayMaxCustomers))
  (bind _currentday (Variables|Default|GetcurrentDay))
  (bind _returnvalue (- _currentday 1))
  (bind _output (Utilities|Array|Get(acopy) _daymaxcustomers _returnvalue))
  (bind _returnvalue_2 (>= _lastcustomerindextoday _output))
  (if _returnvalue_2
    (Variables|Default|SetTurn_Type "NewEnumerator6")
    (Default|CallUIAnimationEventDispatcher)
    (return _returnvalue_2)))

(fn CheckOrder
  (bind _customers (Variables|Default|Getcustomers))
  (bind _returnvalue (Utilities|Array|LastIndex _customers))
  (bind _output (Utilities|Array|Get(acopy) _customers _returnvalue))
  (bind (_desiredfood _desireddrink) (Utilities|Struct|BreakCustomer_struct _output))
  (if (> (Utilities|Array|Length _customers) 0)
    (return (and (== _desiredfood (Variables|Default|GetServingFood)) (== _desireddrink (Variables|Default|GetservedDrink))))))

(fn GetScript
  (params (Script_opening :type Data%20Table%20Object%20Reference) (Script_day1 :type Data%20Table%20Object%20Reference) (Script_day2 :type Data%20Table%20Object%20Reference) (Script_day3 :type Data%20Table%20Object%20Reference))
  (bind _outrownames (DataTable|GetDataTableRowNames Script_opening))
  (for _array_element _outrownames
    (bind _returnvalue (Utilities|GetDataTableRow Script_opening _array_element)
      (:then
        (Utilities|Array|Add (Variables|Default|Getstory_day1_opening) _returnvalue))))
  (bind _outrownames_2 (DataTable|GetDataTableRowNames Script_day1))
  (for _array_element_2 _outrownames_2
    (bind _returnvalue_2 (Utilities|GetDataTableRow Script_day1 _array_element_2)
      (:then
        (Utilities|Array|Add (Variables|Default|Getstory_day1) _returnvalue_2))))
  (bind _outrownames_3 (DataTable|GetDataTableRowNames Script_day2))
  (for _array_element_3 _outrownames_3
    (bind _returnvalue_3 (Utilities|GetDataTableRow Script_day2 _array_element_3)
      (:then
        (Utilities|Array|Add (Variables|Default|Getstory_day2) _returnvalue_3))))
  (bind _outrownames_4 (DataTable|GetDataTableRowNames Script_day3))
  (for _array_element_4 _outrownames_4
    (bind _returnvalue_4 (Utilities|GetDataTableRow Script_day3 _array_element_4)
      (:then
        (Utilities|Array|Add (Variables|Default|Getstory_day3) _returnvalue_4)))))