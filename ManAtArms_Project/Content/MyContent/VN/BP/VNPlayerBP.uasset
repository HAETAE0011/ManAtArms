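; Player Blueprint for a visual-novel food-stall game, managing story and customer turns, their UI widgets and numbered camera switching.
; During gameplay, Tick drains the last customer's satisfaction and counts down the serve cooldown.
; Food and drink events route through Serve to the bartender, then AfterServe restarts cooldown and checks the order.
; Ingredient-based noodle cooking is a debug-print stub, and turn-end and day-limit checks are unwired.
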(event Custom|ChangeCameraTo
  (params (CameraNum :type Integer))
  ;[0 0.3098 1] Camera
  (if (< CameraNum (Variables|Default|GetMaxCamNum))
    (Variables|Default|SetCameraNum CameraNum)
    (Default|CallChangeCameraEventDispatcher)))

(event Custom|UI_Cam
  ;[0 0.3098 1] Camera
  (CallFunction|ChangeCamera)
  (Default|CallChangeCameraEventDispatcher))

(event Custom|coke
  ;[1 0.6497 0.2514] Food Manage
  (CallFunction|Serve "NewEnumerator1" 1))

(event Custom|StartStoryTurn
  ;[0.5781 0.5781 0.5781] Manage Turns
  ;;[1 1 1] Story Mode
  (Utilities|Platform|CollectGarbage)
  (bind _returnvalue (UserInterface|CreateWidget "/Game/MyContent/VN/UI/UI_VN_Story.UI_VN_Story_C" (Game|GetPlayerController 0)))
  (Variables|/Game/MyContent/VN/UI/UI_VN_Story.UI_VN_Story_C|SetPlayer _returnvalue 0)
  (UserInterface|Viewport|AddtoViewport _returnvalue 0)
  (Default|CallUIAnimationEventDispatcher))

(event Custom|beer
  ;[1 0.6497 0.2514] Food Manage
  (CallFunction|Serve "NewEnumerator1" 2))

(event Custom|noodle_1
  ;[1 0.6497 0.2514] Food Manage
  (CallFunction|Serve "NewEnumerator0" 1))

(event Custom|noodle_2
  ;[1 0.6497 0.2514] Food Manage
  (CallFunction|Serve "NewEnumerator0" 2))

(event Custom|ChangeCamera
  ;[0 0.3098 1] Camera
  (if (< (Variables|Default|GetCameraNum) (Variables|Default|GetMaxCamNum))
    (Variables|Default|SetCameraNum (+ (Variables|Default|GetCameraNum) 1))
    (else
      (Variables|Default|SetCameraNum 1))))

(event Custom|skewer_1
  ;[1 0.6497 0.2514] Food Manage
  (CallFunction|Serve "NewEnumerator0" 3))

(event Custom|CustomerTurnStart
  ;[0.5781 0.5781 0.5781] Manage Turns
  ;;[0 0.2626 1] GamePlay
  ;;;[1 0 0] CustomerTurn
  (Variables|Default|SetTurn_type "NewEnumerator5")
  (Default|CallUIAnimationEventDispatcher))

(event Custom|skewer_2
  ;[1 0.6497 0.2514] Food Manage
  (CallFunction|Serve "NewEnumerator0" 4))

(event Custom|StartGameTurn
  ;[0.5781 0.5781 0.5781] Manage Turns
  ;;[0 0.2626 1] GamePlay
  (Variables|Default|SetTurn%20End false)
  (Math|Integer|IncrementInt (Variables|Default|GetCurrentDay)
    (:%20%20
      (Variables|Default|SetMaxCustomerNum (+ (Variables|Default|GetMaxClickNum) (Variables|Default|GetClickNumBonus)))
      (Variables|Default|SetcurrentClickNum 0)
      (Variables|Default|SetTurn_type "NewEnumerator5")
      (bind _returnvalue (UserInterface|CreateWidget "/Game/MyContent/VN/UI/UI_VN_GamePlay_refined.UI_VN_GamePlay_refined_C" (Game|GetPlayerController 0)))
      (Variables|/Game/MyContent/VN/UI/UI_VN_GamePlay_refined.UI_VN_GamePlay_refined_C|SetPlayer _returnvalue 0)
      (UserInterface|Viewport|AddtoViewport _returnvalue 0)
      (CallFunction|ChangeCamerato 1)
      (CallFunction|CustomerTurnStart))))

(event EventBeginPlay
  ;[0.2527 0 1] BeginPlay
  (Variables|Default|SetTurn_type "NewEnumerator1")
  ;;[1 1 1] Call animation : UI
  (Utilities|FlowControl|Delay 0.2)
  (Default|CallUIAnimationEventDispatcher))

(event EventTick
  (params (DeltaSeconds :type Float%20%28single-precision%29))
  ;[0 1 0.005969] On Tick calculations
  (switch Utilities|FlowControl|Switch|SwitchonTurnType (Variables|Default|GetTurn_type)
    (:NewEnumerator0
      ;;[1 0 0] Player making orders
      (CallFunction|StatisfactionLevel DeltaSeconds)
      (CallFunction|HandleCooldown DeltaSeconds))))

(fn ConstructionScript)

(fn AddCustomerF
  (params (name :type String) (food :type Integer) (drink :type Integer))
  (Utilities|Array|Add (Variables|Default|GetCustomers_0) (Utilities|Struct|MakeST_Customer (+ (Utilities|Array|Length (Variables|Default|GetCustomers_0)) 1) name drink food false false false (Variables|Default|Getdefault_satisfaction_level))))

(fn CheckDrink
  (bind _customers_0 (Variables|Default|GetCustomers_0))
  (bind _returnvalue (Utilities|Array|LastIndex _customers_0))
  (bind _output (Utilities|Array|Get(acopy) _customers_0 _returnvalue))
  (Utilities|Struct|SetmembersinST_Customer _output (== (Utilities|Struct|BreakST_Customer _output) (Variables|Default|GetservedDrink))))

(fn CheckFood
  (bind _customers_0 (Variables|Default|GetCustomers_0))
  (bind _returnvalue (Utilities|Array|LastIndex _customers_0))
  (bind _output (Utilities|Array|Get(acopy) _customers_0 _returnvalue))
  (Utilities|Struct|SetmembersinST_Customer _output (== (Utilities|Struct|BreakST_Customer _output) (Variables|Default|GetservedFood)))
  (return))

(fn CheckOrder
  (bind _customers_0 (Variables|Default|GetCustomers_0))
  (bind _returnvalue (Utilities|Array|LastIndex _customers_0))
  (bind _output (Utilities|Array|Get(acopy) _customers_0 _returnvalue))
  (bind (_sat_d _sat_f) (Utilities|Struct|BreakST_Customer _output))
  (bind _structout (Utilities|Struct|SetmembersinST_Customer _output (and _sat_d _sat_f)))
  (return (Utilities|Struct|BreakST_Customer _structout)))

(fn StatisfactionLevel
  (params (delta%20time :type Float%20%28single-precision%29))
  (bind _customers_0 (Variables|Default|GetCustomers_0))
  (bind _returnvalue (Utilities|Array|LastIndex _customers_0))
  (bind _output (Utilities|Array|Get(acopy) _customers_0 _returnvalue))
  (bind _satisfaction_level (Utilities|Struct|BreakST_Customer _output))
  (if (>= _satisfaction_level 0.0)
    (Utilities|Struct|SetmembersinST_Customer _output (- _satisfaction_level (* delta%20time (Variables|Default|GetsatisfactionLv_multiplier))))))

(fn HandleCooldown
  (params (DeltaTime :type Float%20%28single-precision%29))
  (if (not (Variables|Default|GetCooldown_Done))
    (if (> (Variables|Default|GetCooldown) 0.0)
      (Variables|Default|SetCooldown (- (Variables|Default|GetCooldown) DeltaTime))
      (Variables|Default|SetCooldownPercent (/ (Variables|Default|GetCooldown) (Variables|Default|GetCooldown_Max)))
      (else
        (Variables|Default|SetCooldown_Done true)))))

(fn CheckPlayTurnEnd
  (bind _maxclicknum (Variables|Default|GetMaxClickNum))
  (bind _currentclicknum (Variables|Default|GetcurrentClickNum))
  (bind _returnvalue (- _maxclicknum _currentclicknum))
  (bind _returnvalue_2 (<= _returnvalue 0))
  (if _returnvalue_2
    (Variables|Default|SetTurn%20End true)
    (Variables|Default|SetTurn_type "NewEnumerator6")
    (Default|CallUIAnimationEventDispatcher)
    (return _returnvalue_2)))

(fn AfterServe
  (Math|Integer|IncrementInt (Variables|Default|GetcurrentClickNum)
    (:%20%20
      (bind _output_get (Variables|Default|SetCooldown_Max (Variables|cooldown|GetCooldown_f1)))
      (Variables|Default|SetCooldown _output_get)
      (Variables|Default|SetCooldown_Done false)
      (CallFunction|CheckFood)
      (CallFunction|CheckDrink)
      (bind _ordercomplete (CallFunction|CheckOrder))
      ;[1 1 1] if order is completed, reset the order and add new customer
      (if _ordercomplete
        (Variables|Default|SetservedFood 0)
        (Variables|Default|SetservedDrink 0)
        (Development|PrintString "Success")
        (Variables|Default|SetOrderSuccess true)))))

(fn Serve
  (params (serveType :type ServeType%20Enum :default "NewEnumerator0") (typeNum :type Integer))
  (bind _bartender (Variables|Default|GetBartender))
  (Utilities|IsValid _bartender
    (:Is%20Valid
      (Default|GetFood (.AsBP%20Bartender (Utilities|Casting|CastToBP_bartender _bartender)) "serving noodle 1!")
      (switch Utilities|FlowControl|Switch|SwitchonServeType serveType
        (:NewEnumerator0
          (Variables|Default|SetservedFood typeNum))
        (:NewEnumerator1
          (Variables|Default|SetservedDrink typeNum)))
      (CallFunction|AfterServe))))

(fn SetNoodleType
  (params (Index :type Integer))
  (bind _noodletype (Variables|Default|GetNoodleType))
  (for (_ _array_index) _noodletype
    (Utilities|Array|SetArrayElem _noodletype _array_index false))
  (if (Utilities|Array|IsValidIndex _noodletype Index)
    (Utilities|Array|SetArrayElem _noodletype Index true)))

(fn SetSauceType
  (params (Index :type Integer))
  (bind _saucetype (Variables|Default|GetSauceType))
  (for (_ _array_index) _saucetype
    (Utilities|Array|SetArrayElem _saucetype _array_index false))
  (if (Utilities|Array|IsValidIndex _saucetype Index)
    (Utilities|Array|SetArrayElem _saucetype Index true)))

(fn SetToppingType
  (params (Index :type Integer))
  (bind _toppingtype (Variables|Default|GetToppingType))
  (for (_ _array_index) _toppingtype
    (Utilities|Array|SetArrayElem _toppingtype _array_index false))
  (if (Utilities|Array|IsValidIndex _toppingtype Index)
    (Utilities|Array|SetArrayElem _toppingtype Index true)))

(fn CookNoodle
  (bind _toppingtype (Variables|Default|GetToppingType))
  (bind _noodletype (Variables|Default|GetNoodleType))
  (bind _noodletype_2 (Variables|Default|GetNoodleType))
  (bind _saucetype (Variables|Default|GetSauceType))
  ;[1 1 1] Check If ingredients are not empty
  (Variables|Default|Setn_noodle_count 0)
  (Variables|Default|Setn_sauce_count 0)
  (Variables|Default|Setn_topping_count 0)
  ;;[1 1 1] Check Noodle
  (for _index (range 0 (- (Utilities|Array|Length _noodletype_2) 1))
    (if (Utilities|Array|Get(acopy) _noodletype_2 _index)
      (Math|Integer|IncrementInt (Variables|Default|Getn_noodle_count))))
  (if (> (Variables|Default|Getn_noodle_count) 0)
    ;;[1 1 1] Check Sauce
    (for _index_2 (range 0 (- (Utilities|Array|Length _saucetype) 1))
      (if (Utilities|Array|Get(acopy) _saucetype _index_2)
        (Math|Integer|IncrementInt (Variables|Default|Getn_sauce_count))))
    (if (> (Variables|Default|Getn_sauce_count) 0)
      ;;[1 1 1] Check Toppings
      (for _index_3 (range 0 (- (Utilities|Array|Length _toppingtype) 1))
        (if (Utilities|Array|Get(acopy) _toppingtype _index_3)
          (Math|Integer|IncrementInt (Variables|Default|Getn_topping_count))))
      (if (> (Variables|Default|Getn_topping_count) 0)
        (if (or (> (Variables|Default|Getn_noodle_count) 1) (> (Variables|Default|Getn_sauce_count) 1))
          (Development|PrintString "Using more than one Noodle or Sauce!")
          (else
            (for _index_4 (range 0 (- (Utilities|Array|Length _noodletype) 1))
              (if (Utilities|Array|Get(acopy) _noodletype _index_4)
                (switch int _index_4
                  (:0
                    (if (Utilities|Array|Get(acopy) (Variables|Default|GetSauceType) 1)
                      ;[1 1 1] make SeafoodNoodle
                      (if (Utilities|Array|Get(acopy) (Variables|Default|GetToppingType))
                        (Development|PrintString "SEAFOOD NOODLE"))
                      (elif true
                        _))))))))))))