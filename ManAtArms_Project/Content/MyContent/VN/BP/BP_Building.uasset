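; Procedural building actor that generates stacked floors of wall meshes along an editable spline outline, entirely in the Construction Script.
; Each floor repeats the outline at FloorHeight intervals with linear spline meshes, subdividing long segments through temporary splines.
; A procedural mesh ceiling is built as a triangle fan from the actor origin at Height.
; Random mesh selection and SplineMeshCreation are not used by the live construction path.
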(event EventBeginPlay)

(event Collision|EventActorBeginOverlap
  (params (OtherActor :type Actor%20Object%20Reference)))

(event EventTick
  (params (DeltaSeconds :type Float%20%28single-precision%29)))

(fn ConstructionScript
  (bind _spline (Variables|Default|GetSpline))
  (bind _ceiling (Variables|Default|GetCeiling))
  (bind _spline_2 (Variables|Default|GetSpline))
  (bind _returnvalue (Spline|GetNumberOfSplinePoints _spline))
  (bind _returnvalue_2 (- _returnvalue 1))
  ;[1 1 1] Refresh function
  (if (Variables|Base|GetRefresh)
    (Class|KismetMathLibrary|SeedRandomStream (Variables|Default|GetStream))
    (Variables|Base|SetRefresh false))
  (Utilities|FlowControl|Sequence
    (:then_0
      ;[1 1 1] Floors
      (for _index (range 0 (- (Variables|Default|GetNumberOfFloors) 1))
        ;[1 1 1] For each point of spline
        (for _index_2 (range 0 _returnvalue_2)
          (if (not (== _index_2 _returnvalue_2))
            (if (< (.ReturnValue2 (|CheckTheLength _spline _index_2 _spline _index_2)) 1)
              (Spline|SetSplinePointType _spline _index_2 "Linear" true)
              (bind _returnvalue_3 (AddComponent|AddSplineMeshComponent false))
              (SplineMesh|SetForwardAxis _returnvalue_3 (Variables|Default|GetForwardAxis) true)
              (Components|StaticMesh|SetStaticMesh _returnvalue_3 (Variables|Meshes|GetMesh))
              (SplineMesh|SetStartandEnd _returnvalue_3 (+ (Spline|GetLocationatSplinePoint _spline _index_2 "Local") (Math|Vector|MakeVector 0.0 0.0 (* (Variables|Default|GetfloorHeight) (Math|Conversions|ToFloat(Integer) _index)))) (Spline|GetTangentatSplinePoint _spline _index_2 "Local") (+ (Spline|GetLocationatSplinePoint _spline (+ _index_2 1) "Local") (Math|Vector|MakeVector 0.0 0.0 (* (Variables|Default|GetfloorHeight) (Math|Conversions|ToFloat(Integer) _index)))) (Spline|GetTangentatSplinePoint _spline _index_2 "Local") true :!class /Script/Engine.SplineMeshComponent)
              (else
                (bind _returnvalue_4 (AddComponent|AddSplineComponent false))
                (Spline|ClearSplinePoints _returnvalue_4 true)
                (for _index_3 (range 0 (.ReturnValue2 (|CheckTheLength _spline _index_2 _spline _index_2)))
                  (Spline|AddSplinePoint _returnvalue_4 (Spline|GetLocationatDistanceAlongSpline _spline (+ (Spline|GetDistanceAlongSplineatSplinePoint _spline _index_2) (* _index_3 (/ (.ReturnValue (|CheckTheLength _spline _index_2 _spline _index_2)) (Math|Conversions|ToFloat(Integer) (.ReturnValue2 (|CheckTheLength _spline _index_2 _spline _index_2)))))) "World") "World" true))
                (for _index_4 (range 0 (.ReturnValue2 (|CheckTheLength _spline _index_2 _spline _index_2)))
                  (Spline|SetSplinePointType _returnvalue_4 _index_4 "Linear" true)
                  (bind _returnvalue_5 (AddComponent|AddSplineMeshComponent false))
                  (SplineMesh|SetForwardAxis _returnvalue_5 (Variables|Default|GetForwardAxis) true)
                  (Components|StaticMesh|SetStaticMesh _returnvalue_5 (Variables|Meshes|GetMesh))
                  (SplineMesh|SetStartandEnd _returnvalue_5 (+ (Spline|GetLocationatSplinePoint _returnvalue_4 _index_4 "Local") (Math|Vector|MakeVector 0.0 0.0 (* (Variables|Default|GetfloorHeight) (Math|Conversions|ToFloat(Integer) _index)))) (Spline|GetTangentatSplinePoint _returnvalue_4 _index_4 "Local") (+ (Spline|GetLocationatSplinePoint _returnvalue_4 (+ _index_4 1) "Local") (Math|Vector|MakeVector 0.0 0.0 (* (Variables|Default|GetfloorHeight) (Math|Conversions|ToFloat(Integer) _index)))) (Spline|GetTangentatSplinePoint _returnvalue_4 _index_4 "Local") true :!class /Script/Engine.SplineMeshComponent))
                (Spline|ClearSplinePoints _returnvalue_4 true)))))))
    (:then_1
      ;[1 1 1] Procedurally generated ceiling
      (Variables|Default|SetheightSuggestion (* (Variables|Default|GetNumberOfFloors) (Variables|Default|GetfloorHeight)))
      (for _index_5 (range 0 (- (Spline|GetNumberOfSplinePoints _spline_2) 1))
        (Class|ProceduralMeshComponent|CreateMeshSectionLinearColor _ceiling _index_5 (Utilities|Array|MakeArray (Math|Vector|MakeVector 0.0 0.0 (Variables|Default|Getheight)) (+ (Spline|GetLocationatSplinePoint _spline_2 _index_5 "Local") (Math|Vector|MakeVector 0.0 0.0 (Variables|Default|Getheight))) (+ (Spline|GetLocationatSplinePoint _spline_2 (+ _index_5 1) "Local") (Math|Vector|MakeVector 0.0 0.0 (Variables|Default|Getheight)))) (Utilities|Array|MakeArray 0 1 2) 0 (Utilities|Array|MakeArray "" "(X=0.000000,Y=1.000000)" "(X=1.000000,Y=0.000000)" "(X=1.000000,Y=1.000000)") 0 0 0 0 0 true)
        (Rendering|Material|SetMaterial _ceiling _index_5 (Variables|Default|GetCeilingMaterial))))))

(fn SplineMeshCreation
  (params (Spline :type Spline%20Component%20Object%20Reference) (Start :type Static%20Mesh%20Object%20Reference) (Middle :type Static%20Mesh%20Object%20Reference) (End :type Static%20Mesh%20Object%20Reference))
  (bind _returnvalue (Spline|GetNumberOfSplinePoints Spline))
  (bind _returnvalue_2 (- _returnvalue 2))
  ;[1 1 1] Spline Mesh
  (for _index (range 0 _returnvalue_2)
    (bind _returnvalue_3 (AddComponent|AddSplineMeshComponent false))
    (if (== _index 0)
      ;;[1 0.4688 0.4688] Three Meshes- start, middle, end
      (Components|StaticMesh|SetStaticMesh _returnvalue_3 Start)
      (elif (== _returnvalue_2 _index)
        (Components|StaticMesh|SetStaticMesh _returnvalue_3 End)
        (else
          (Components|StaticMesh|SetStaticMesh _returnvalue_3 Middle))))
    (SplineMesh|SetStartandEnd _returnvalue_3 (Spline|GetLocationatSplinePoint Spline _index "Local") (Spline|GetTangentatSplinePoint Spline _index "Local") (Spline|GetLocationatSplinePoint Spline (+ _index 1) "Local") (Spline|GetTangentatSplinePoint Spline (+ _index 1) "Local") true :!class /Script/Engine.SplineMeshComponent)))