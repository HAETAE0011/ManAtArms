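; Decal actor Blueprint that passes its orientation to its decal material.
; The construction script creates a dynamic instance of the chosen material, assigns it to the decal and writes rotation axes into vector parameters, with X and Z swapped.
; A Refresh boolean resets itself on construction, acting as an editor update toggle.
; The event graph is unused, so nothing updates at runtime.
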(event EventBeginPlay)

(event Collision|EventActorBeginOverlap
  (params (OtherActor :type Actor%20Object%20Reference)))

(event EventTick
  (params (DeltaSeconds :type Float%20%28single-precision%29)))

(fn ConstructionScript
  (bind _returnvalue (Transformation|GetActorRotation))
  (bind (_x _y _z) (Math|Rotator|BreakRotIntoAxes _returnvalue))
  ;[1 1 1] Refresh function
  (if (Variables|Default|GetRefresh)
    (Variables|Default|SetRefresh false))
  (bind _returnvalue_2 (Rendering|Material|CreateDynamicMaterialInstance (Variables|Default|GetMat) "None" :!class /Script/Engine.KismetMaterialLibrary))
  (Rendering|Components|Decal|SetDecalMaterial (Variables|Default|GetDecal) _returnvalue_2)
  (Rendering|Material|SetVectorParameterValue _returnvalue_2 "X" (Math|Conversions|ToLinearColor(Vector) _z) :!class /Script/Engine.MaterialInstanceDynamic)
  (Rendering|Material|SetVectorParameterValue _returnvalue_2 "Y" (Math|Conversions|ToLinearColor(Vector) _y) :!class /Script/Engine.MaterialInstanceDynamic)
  (Rendering|Material|SetVectorParameterValue _returnvalue_2 "Z" (Math|Conversions|ToLinearColor(Vector) _x) :!class /Script/Engine.MaterialInstanceDynamic))